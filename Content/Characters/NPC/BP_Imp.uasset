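; Guardian imp NPC that patrols random custom targets or watched torches and runs to extinguish torches that need help.
; TorchNeedsHelp and TorchIsOkay maintain a help queue that switches it between patrol and help speeds, using AIMoveTo.
; A BP_TestWeapon hit hides it and spawns a mask, where it respawns after a random delay.
; The construction script prunes torches not listing it as guardian and draws debug lines to patrol targets.
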(event `self.ReceiveBeginPlay`
  (set `CharacterMovementComponent.MaxWalkSpeed` (`self.PatrollingSpeed`) (`self.CharacterMovement`))
  (bind (_array_element _array_index) (`/Game/Gameplay/BPML_CustomMacros.ReverseForEachLoop` (`self.CustomTargets`))
    (:`LoopBody`
      (`/Engine/EditorBlueprintResources/StandardMacros.IsValid` _array_element
        (:`Is Not Valid`
          (`KismetArrayLibrary.Array_Remove` (`self.CustomTargets`) _array_index))))
    (:`Completed`
      (if (!= (`KismetArrayLibrary.Array_Length` (`self.CustomTargets`)) 0)
        (`KismetSystemLibrary.Delay` 0.42 :!label _label)
        (if (== (`KismetArrayLibrary.Array_Length` (`self.TorchesNeedingHelp`)) 0)
          (set `CharacterMovementComponent.MaxWalkSpeed` (`self.PatrollingSpeed`) (`self.CharacterMovement`))
          (`self.Patrol`))
        (else
          (set `self.UseCustomTargets` false)
          (if (!= (`KismetArrayLibrary.Array_Length` (`self.DoNotEditThisArray_TorchesToWatch`)) 0)
            (goto _label)
            (else
              (`KismetSystemLibrary.PrintString` "My life is pointless ;_;"))))))))

(event `Patrol`
  (bind _donoteditthisarray_torchestowatch (`self.DoNotEditThisArray_TorchesToWatch`))
  (bind _customtargets (`self.CustomTargets`))
  (if (`self.IsDead`)
    _
    (elif (`self.UseCustomTargets`)
      (`|AIMoveTo` self (0.0 0.0 0.0) (`KismetArrayLibrary.Array_Get` _customtargets (`self.DestinationIndex`)) (`self.PatrolErrorRadius`)
        (:`OnSuccess`
          (`KismetSystemLibrary.Delay` (`KismetMathLibrary.RandomFloatInRange` (`self.MinPatrolPause`) (`self.MaxPatrolPause`))))
        (:`OnFail`
          _))
      (set `self.DestinationToTry` (`KismetMathLibrary.RandomIntegerInRange` 0 (- (`KismetArrayLibrary.Array_Length` _customtargets) 1)) :!label _label_2)
      (if (!= (`self.DestinationIndex`) (`self.DestinationToTry`))
        (set `self.DestinationIndex` (`self.DestinationToTry`))
        (if (`self.IsPatrolling`)
          (if (not (`self.IsDead`))
            (`self.Patrol`)))
        (else
          (goto _label_2)))
      (else
        (`|AIMoveTo` self (0.0 0.0 0.0) (`KismetArrayLibrary.Array_Get` _donoteditthisarray_torchestowatch (`self.DestinationIndex`)) (`self.PatrolErrorRadius`)
          (:`OnSuccess`
            (`KismetSystemLibrary.Delay` (`KismetMathLibrary.RandomFloatInRange` (`self.MinPatrolPause`) (`self.MaxPatrolPause`))))
          (:`OnFail`
            _))
        (set `self.DestinationToTry` (`KismetMathLibrary.RandomIntegerInRange` 0 (- (`KismetArrayLibrary.Array_Length` _donoteditthisarray_torchestowatch) 1)) :!label _label_3)
        (if (!= (`self.DestinationIndex`) (`self.DestinationToTry`))
          (set `self.DestinationIndex` (`self.DestinationToTry`))
          (if (`self.IsPatrolling`)
            (if (not (`self.IsDead`))
              (`self.Patrol`)))
          (else
            (goto _label_3)))))))

(event `self.ReceiveActorBeginOverlap`
  (params (OtherActor :type "Actor Object Reference"))
  (bind _asbp_test_weapon (cast `/Game/Weapons/BP_TestWeapon` OtherActor))
  (if (`/Game/Weapons/BP_TestWeapon.CanKillImp` _asbp_test_weapon)
    (set `/Game/Weapons/BP_TestWeapon.CanKillImp` false _asbp_test_weapon)
    (`self.Die`)))

(event `Die`
  (set `self.IsDead` true)
  (`NavMovementComponent.StopActiveMovement` (`self.CharacterMovement`))
  (`self.SetActorEnableCollision` false)
  (`self.SetActorHiddenInGame` true)
  (`GameplayStatics.SpawnEmitterAtLocation` "/Game/HDParticlePack/Particles/P_AtomHyper.P_AtomHyper" (`self.K2_GetActorLocation`))
  (bind _returnvalue (`|SpawnActorFromClass` "/Game/Characters/NPC/BP_ImpMask.BP_ImpMask_C" (`self.GetTransform`) "Undefined" "OverrideRootScale"))
  (set `self.Mask` _returnvalue)
  (`self.SetActorTickEnabled` false)
  (`KismetSystemLibrary.Delay` (`KismetMathLibrary.RandomFloatInRange` (`self.MinRespawnTime`) (`self.MaxRespawnTime`)))
  (`self.Respawn`))

(event `Respawn`
  (bind _mask (`self.Mask`))
  (bind _returnvalue (`self.K2_GetActorLocation` _mask))
  (`GameplayStatics.SpawnEmitterAtLocation` "/Game/HDParticlePack/Particles/P_AtomHyper.P_AtomHyper" _returnvalue)
  (`self.K2_SetActorLocationAndRotation` _returnvalue (`KismetMathLibrary.MakeRotator` 0.0 0.0 (.yaw (`self.K2_GetActorRotation` _mask))))
  (`self.K2_DestroyActor` (`self.Mask`))
  (`self.SetActorHiddenInGame` false)
  (`self.SetActorEnableCollision` true)
  (`self.SetActorTickEnabled` true)
  (set `self.IsDead` false)
  (if (== (`KismetArrayLibrary.Array_Length` (`self.TorchesNeedingHelp`)) 0)
    (set `self.IsPatrolling` true)
    (set `CharacterMovementComponent.MaxWalkSpeed` (`self.PatrollingSpeed`) (`self.CharacterMovement`))
    (`self.Patrol`)
    (else
      (set `self.IsPatrolling` false)
      (set `CharacterMovementComponent.MaxWalkSpeed` (`self.HelpingSpeed`) (`self.CharacterMovement`))
      (`self.HelpTorch`))))

(event `TorchNeedsHelp`
  (params (Torch :type "/Game/Gameplay/Torches/BP_TorchBase Object Reference"))
  (`KismetArrayLibrary.Array_AddUnique` (`self.TorchesNeedingHelp`) Torch)
  (set `self.IsPatrolling` false)
  (set `CharacterMovementComponent.MaxWalkSpeed` (`self.HelpingSpeed`) (`self.CharacterMovement`))
  (`self.HelpTorch`))

(event `HelpTorch`
  (if (not (`self.IsDead`))
    (bind _output_get (set `self.CurrentTorchToHelp` (`KismetArrayLibrary.Array_Get` (`self.TorchesNeedingHelp`))))
    (`|AIMoveTo` self (0.0 0.0 0.0) _output_get (`self.HelpErrorRadius`)
      (:`OnSuccess`
        (`KismetSystemLibrary.PrintString` (`KismetStringLibrary.Concat_StrStr` "I defended " (`KismetSystemLibrary.GetDisplayName` _output_get) "!"))
        (if (`KismetArrayLibrary.Array_Contains` (`self.TorchesNeedingHelp`) (`self.CurrentTorchToHelp`))
          (`self.Jump`)
          (`/Game/Gameplay/Torches/BP_TorchBase.ExtinguishFire` (`self.CurrentTorchToHelp`))
          (elif (!= (`KismetArrayLibrary.Array_Length` (`self.TorchesNeedingHelp`)) 0)
            (set `self.IsPatrolling` false)
            (set `CharacterMovementComponent.MaxWalkSpeed` (`self.HelpingSpeed`) (`self.CharacterMovement`))
            (`self.HelpTorch`)
            (else
              (set `self.IsPatrolling` true)
              (set `CharacterMovementComponent.MaxWalkSpeed` (`self.PatrollingSpeed`) (`self.CharacterMovement`))
              (`self.Patrol`)))))
      (:`OnFail`
        (`KismetSystemLibrary.PrintString` (`KismetStringLibrary.Concat_StrStr` "I can't defend " (`KismetSystemLibrary.GetDisplayName` _output_get) " :("))))))

(event `TorchIsOkay`
  (params (Torch :type "/Game/Gameplay/Torches/BP_TorchBase Object Reference"))
  (bind _torchesneedinghelp (`self.TorchesNeedingHelp`))
  (`KismetArrayLibrary.Array_RemoveItem` _torchesneedinghelp Torch)
  (if (!= (`KismetArrayLibrary.Array_Length` _torchesneedinghelp) 0)
    (set `self.IsPatrolling` false)
    (set `CharacterMovementComponent.MaxWalkSpeed` (`self.HelpingSpeed`) (`self.CharacterMovement`))
    (`self.HelpTorch`)
    (else
      (set `self.IsPatrolling` true)
      (set `CharacterMovementComponent.MaxWalkSpeed` (`self.PatrollingSpeed`) (`self.CharacterMovement`))
      (`self.Patrol`))))

(fn `UserConstructionScript`
  (bind _donoteditthisarray_torchestowatch (`self.DoNotEditThisArray_TorchesToWatch`))
  (`PrimitiveComponent.SetWalkableSlopeOverride` (`self.CapsuleComponent`) (make `WalkableSlopeOverride` "WalkableSlope_Unwalkable" 0.0))
  (bind _outactors (`GameplayStatics.GetAllActorsOfClass` "/Game/Gameplay/Torches/BP_TorchBase.BP_TorchBase_C"))
  (bind _array_element (`/Game/Gameplay/BPML_CustomMacros.ReverseForEachLoop` _outactors)
    (:`LoopBody`
      (if (and (`KismetArrayLibrary.Array_Contains` _donoteditthisarray_torchestowatch _array_element) (not (`KismetArrayLibrary.Array_Contains` (`/Game/Gameplay/Torches/BP_TorchBase.GuardianImps` _array_element) self)))
        (`KismetArrayLibrary.Array_RemoveItem` _donoteditthisarray_torchestowatch _array_element)))
    (:`Completed`
      (`KismetSystemLibrary.FlushPersistentDebugLines`)
      (if (`self.UseCustomTargets`)
        (for _array_element_2 (`self.CustomTargets`)
          (`/Engine/EditorBlueprintResources/StandardMacros.IsValid` _array_element_2
            (:`Is Valid`
              (`KismetSystemLibrary.DrawDebugLine` (`self.K2_GetActorLocation`) (`self.K2_GetActorLocation` _array_element_2) (struct :`R` 0.5 :`B` 1.0 :`A` 1.0) 61440.0 2.8))))
        (else
          (for _array_element_3 (`self.DoNotEditThisArray_TorchesToWatch`)
            (`KismetSystemLibrary.DrawDebugLine` (`self.K2_GetActorLocation`) (`self.K2_GetActorLocation` _array_element_3) (struct :`R` 0.5 :`B` 1.0 :`A` 1.0) 61440.0 2.8)))))))