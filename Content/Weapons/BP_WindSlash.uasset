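; BP_WindSlash is a wind slash weapon projectile that destroys itself once its Lifetime elapses after BeginPlay.
; Its construction script adds PlayerSpeed to the ProjectileMovement initial speed and caps max speed at that same value.
; The Destroy event is empty, and nodes for an effect fade-out delay and RangeMultiplier-based lifetime scaling are present but never run.
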(event `self.ReceiveBeginPlay`
  (`KismetSystemLibrary.Delay` (`self.Lifetime`))
  (`self.K2_DestroyActor`))

(event `Destroy`)

(fn `UserConstructionScript`
  (bind _projectilemovement (`self.ProjectileMovement`))
  (bind _output_get (set `ProjectileMovementComponent.InitialSpeed` (+ (`ProjectileMovementComponent.InitialSpeed` (`self.ProjectileMovement`)) (`self.PlayerSpeed`)) _projectilemovement))
  (set `ProjectileMovementComponent.MaxSpeed` _output_get _projectilemovement))