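; BP_UmaySensor is a one-time story trigger that fires when the player overlaps it at the required Progress value.
; It disables input, advances Progress, spawns windstone particles at the player's Fan and streams in the listed levels one after another.
; It then blends to a cutscene camera, turns Umay 90 degrees in yaw with a timeline, and blends back to the player before restoring input.
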(event `/Game/Gameplay/SpecialCaseTriggers/BP_DoorSensor.ReceiveActorBeginOverlap`
  (params (OtherActor :type "Actor Object Reference"))
  (bind _startz_rotation (`self.StartZ_Rotation`))
  (bind _umay (`self.Umay`))
  (bind _asthird_person_character (cast `/Game/Characters/Player/ThirdPersonCharacter` (`GameplayStatics.GetPlayerCharacter` 0) :!pure true))
  (bind _asthird_person_character_2 (cast `/Game/Characters/Player/ThirdPersonCharacter` OtherActor))
  (if (`|EnumEquality` (`/Game/Characters/Player/ThirdPersonCharacter.Progress` _asthird_person_character_2) (`self.ProgressNeeded`))
    (`/Engine/EditorBlueprintResources/StandardMacros.DoOnce` false
      (:`Completed`
        (set `self.StartZ_Rotation` (.yaw (`self.K2_GetActorRotation` (`self.Umay`))))
        (`self.DisableInput` _asthird_person_character (`GameplayStatics.GetPlayerController` 0))
        (set `/Game/Characters/Player/ThirdPersonCharacter.Progress` (`self.ProgressToSet`) _asthird_person_character)
        (for _ (range 1 (+ (`self.NumPowerParticles`) 1))
          (`|SpawnActorFromClass` "/Game/Gameplay/BP_WindstoneParticles.BP_WindstoneParticles_C" (`KismetMathLibrary.MakeTransform` (`SceneComponent.K2_GetComponentLocation` (`/Game/Characters/Player/ThirdPersonCharacter.Fan` _asthird_person_character))) "Undefined" "OverrideRootScale"))
        (if (< (`self.LevelIterator`) (`KismetArrayLibrary.Array_Length` (`self.LevelsToLoad`))) :!label _label
          (`GameplayStatics.LoadStreamLevel` (`KismetArrayLibrary.Array_Get` (`self.LevelsToLoad`) (`self.LevelIterator`)) true)
          (`/Engine/EditorBlueprintResources/StandardMacros.IncrementInt` (`self.LevelIterator`)
            (:`  `
              (goto _label)))
          (else
            (`PlayerController.SetViewTargetWithBlend` (`GameplayStatics.GetPlayerController` 0) (`self.CutsceneCamera`) 4.2 "VTBlend_EaseInOut" 4.0 false)
            (`KismetSystemLibrary.Delay` 4.2)
            (bind (_direction _rotationtrack) (`Timeline|RotationGraph` :!via `PlayFromStart`)
              (:`Update`
                (`self.SetActorRotation` _umay (`KismetMathLibrary.MakeRotator` (.roll (`self.K2_GetActorRotation` _umay)) (.pitch (`self.K2_GetActorRotation` _umay)) (`KismetMathLibrary.Lerp` _startz_rotation (`KismetMathLibrary.NormalizeAxis` (+ _startz_rotation 90.0)) _rotationtrack))))
              (:`Finished`
                (`PlayerController.SetViewTargetWithBlend` (`GameplayStatics.GetPlayerController` 0) (cast `/Game/Characters/Player/ThirdPersonCharacter` (`GameplayStatics.GetPlayerCharacter` 0) :!pure true) 4.2 "VTBlend_EaseInOut" 4.0 false)
                (`KismetSystemLibrary.Delay` 4.2)
                (`self.EnableInput` (cast `/Game/Characters/Player/ThirdPersonCharacter` (`GameplayStatics.GetPlayerCharacter` 0) :!pure true) (`GameplayStatics.GetPlayerController` 0))))))))))

(fn `UserConstructionScript`)