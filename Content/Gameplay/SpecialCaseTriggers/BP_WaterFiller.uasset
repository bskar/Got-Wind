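; BP_WaterFiller is a one-shot trigger that raises or moves a water actor when Vayu overlaps it at a specific progress stage.
; On overlap it checks the BP_Vayu Progress enum, then a DoOnce disables Vayu movement.
; A FillGraph timeline lerps the referenced Water actor from its current location to EndLocation, and movement is re-enabled when the timeline finishes.
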(event `self.ReceiveActorBeginOverlap`
  (params (OtherActor :type "Actor Object Reference"))
  (bind _asbp_vayu (cast `/Game/Characters/Player/BP_Vayu` OtherActor))
  (if (`|EnumEquality` (`/Game/Characters/Player/BP_Vayu.Progress` _asbp_vayu) "NewEnumerator5")
    (`/Engine/EditorBlueprintResources/StandardMacros.DoOnce` false
      (:`Completed`
        (`/Game/Characters/Player/BP_Vayu.DisableVayuMovement` _asbp_vayu)
        (set `self.StartLocation` (`self.K2_GetActorLocation` (`self.Water`)))
        (bind (_direction _filltrack) (`Timeline|FillGraph` :!via `PlayFromStart`)
          (:`Update`
            (`self.K2_SetActorLocation` (`self.Water`) (`KismetMathLibrary.VLerp` (`self.StartLocation`) (`self.EndLocation`) _filltrack) false false))
          (:`Finished`
            (`/Game/Characters/Player/BP_Vayu.EnableVayuMovement` _asbp_vayu)))))))

(fn `UserConstructionScript`)