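; Trigger actor that opens or closes a referenced door once, when the ThirdPersonCharacter overlaps it with Progress exactly matching ProgressNeeded.
; A timeline lerps the door's Z from its starting height up or down by OpenCloseDistance, using a separate track for each MovementDirection.
; When the movement finishes, it unloads any streamed levels listed in LevelsToUnload.
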(event `self.ReceiveActorBeginOverlap`
  (params (OtherActor :type "Actor Object Reference"))
  (bind _door (`self.Door`))
  (bind _asthird_person_character (cast `/Game/Characters/Player/ThirdPersonCharacter` OtherActor))
  (if (`|EnumEquality` (`/Game/Characters/Player/ThirdPersonCharacter.Progress` _asthird_person_character) (`self.ProgressNeeded`))
    (`/Engine/EditorBlueprintResources/StandardMacros.DoOnce` false
      (:`Completed`
        (set `self.StartZ_Position` (.z (`self.K2_GetActorLocation` (`self.Door`))))
        (bind (_direction _uptrack _downtrack) (`Timeline|UpOrDownGraph` :!via `PlayFromStart`)
          (:`Update`
            (switch `EScrollDirection` (`self.MovementDirection`)
              (:`Scroll_Down`
                (`self.K2_SetActorLocation` (`self.Door`) (`KismetMathLibrary.MakeVector` (.x (`self.K2_GetActorLocation` (`self.Door`))) (.y (`self.K2_GetActorLocation` (`self.Door`))) (`KismetMathLibrary.Lerp` (`self.StartZ_Position`) (- (`self.StartZ_Position`) (`self.OpenCloseDistance`)) _downtrack)) false false))
              (:`Scroll_Up`
                (`self.K2_SetActorLocation` _door (`KismetMathLibrary.MakeVector` (.x (`self.K2_GetActorLocation` _door)) (.y (`self.K2_GetActorLocation` _door)) (`KismetMathLibrary.Lerp` (`self.StartZ_Position`) (+ (`self.StartZ_Position`) (`self.OpenCloseDistance`)) _uptrack)) false false))))
          (:`Finished`
            (if (!= (`KismetArrayLibrary.Array_Length` (`self.LevelsToUnload`)) 0)
              (for _array_element (`self.LevelsToUnload`)
                (`GameplayStatics.UnloadStreamLevel` _array_element)))))))))

(fn `UserConstructionScript`)