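; BP_AmbienceTransitionTrigger is a trigger actor that switches ambience when BP_Vayu overlaps it.
; On overlap it compares Vayu's CurrentAmbience with its own AmbienceToStart and skips the switch if they already match.
; Otherwise it updates CurrentAmbience and calls AmbienceTransition on Vayu, passing the ambiences to stop and start with their fade-out and fade-in times.
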(event `self.ReceiveBeginPlay`)

(event `self.ReceiveActorBeginOverlap`
  (params (OtherActor :type "Actor Object Reference"))
  (bind _asbp_vayu (cast `/Game/Characters/Player/BP_Vayu` OtherActor))
  (if (`|EnumInequality` (`/Game/Characters/Player/BP_Vayu.CurrentAmbience` _asbp_vayu) (`self.AmbienceToStart`))
    (set `/Game/Characters/Player/BP_Vayu.CurrentAmbience` (`self.AmbienceToStart`) _asbp_vayu)
    (`/Game/Characters/Player/BP_Vayu.AmbienceTransition` _asbp_vayu (`self.AmbienceToStop`) (`self.FadeOutTime`) (`self.AmbienceToStart`) (`self.FadeInTime`))))

(fn `UserConstructionScript`)