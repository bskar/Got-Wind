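; BP_ChimeSoundTrigger is a trigger actor that plays a chime when Vayu superjumps upward through it.
; On overlap it casts to BP_Vayu, checks the superjump flag and upward velocity, then activates the ChimeSound component with a reset.
; An unconnected stop-and-replay branch for the chime is left unused in the graph.
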(event `self.ReceiveActorBeginOverlap`
  (params (OtherActor :type "Actor Object Reference"))
  (bind _asbp_vayu (cast `/Game/Characters/Player/BP_Vayu` OtherActor))
  (if (and (`/Game/Characters/Player/BP_Vayu.IsSuperjumping` _asbp_vayu) (> (.z (`self.GetVelocity` _asbp_vayu)) 4.0))
    (`ActorComponent.SetActive` (`self.ChimeSound`) true true)))

(fn `UserConstructionScript`)