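; Spin platform that toggles a linked gate when the third-person character presses Spin while overlapping it.
; Overlap events set CanActivate, and a press only counts if the character is not already spinning or slashing.
; Each activation fires the platform effect and alternately snaps the gate up or down via FlipFlop.
; A DoOnce with delayed reset enforces a cooldown, and clearing CanActivate requires re-entering before the next use.
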(event `self.ReceiveActorBeginOverlap`
  (params (OtherActor :type "Actor Object Reference"))
  (cast `/Game/Dev/ThirdPersonBP/Blueprints/ThirdPersonCharacter` OtherActor)
  (set `self.CanActivate` true))

(event `self.ReceiveActorEndOverlap`
  (params (OtherActor :type "Actor Object Reference"))
  (cast `/Game/Dev/ThirdPersonBP/Blueprints/ThirdPersonCharacter` OtherActor)
  (set `self.CanActivate` false))

(event `InputAction|Spin` :consume false
  (params (Key :type "Key Structure" :default "AnyKey"))
  (:`Pressed`
    (if (`self.CanActivate`)
      (bind _asthird_person_character (cast `/Game/Dev/ThirdPersonBP/Blueprints/ThirdPersonCharacter` (`GameplayStatics.GetPlayerCharacter` 0)))
      (if (not (or (`/Game/Dev/ThirdPersonBP/Blueprints/ThirdPersonCharacter.IsSpinning` _asthird_person_character) (`/Game/Dev/ThirdPersonBP/Blueprints/ThirdPersonCharacter.IsSlashing` _asthird_person_character)))
        (`/Engine/EditorBlueprintResources/StandardMacros.DoOnce` false :!label _label
          (:`Completed`
            (set `self.CanActivate` false)
            (`ActorComponent.Activate` (`self.SpinnyPlatformEffect`) false)
            (`/Engine/EditorBlueprintResources/StandardMacros.FlipFlop`
              (:`A`
                (`self.K2_AddActorLocalOffset` (`self.Gate`) (0.0 0.0 420.0) false false))
              (:`B`
                (`self.K2_AddActorLocalOffset` (`self.Gate`) (0.0 0.0 -420.0) false false)))
            (`KismetSystemLibrary.Delay` 2.0)
            (goto _label :!via `Reset`)))))))

(fn `UserConstructionScript`)