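; Base actor for puzzle objects that activate when all their linked torches are on fire, with an empty Activate event as the hook for the response.
; AddOneTorch and SubtractOneTorch track the lit count, and reaching the required number calls Activate.
; The required number comes from the linked torch array, pruned of invalid entries on construction and BeginPlay.
; The construction script also draws long-lived debug lines to each torch to visualize the links.
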(event `self.ReceiveBeginPlay`
  (bind _donoteditthisarray_torchesneeded (`self.DoNotEditThisArray_TorchesNeeded`))
  (bind (_array_element _array_index) (`/Game/Gameplay/BPML_CustomMacros.ReverseForEachLoop` _donoteditthisarray_torchesneeded)
    (:`LoopBody`
      (`/Engine/EditorBlueprintResources/StandardMacros.IsValid` _array_element
        (:`Is Not Valid`
          (`KismetArrayLibrary.Array_Remove` _donoteditthisarray_torchesneeded _array_index))))
    (:`Completed`
      (set `self.NumTorchesNeeded` (`KismetArrayLibrary.Array_Length` (`self.DoNotEditThisArray_TorchesNeeded`))))))

(event `AddOneTorch`
  (bind _result (`/Engine/EditorBlueprintResources/StandardMacros.IncrementInt` (`self.NumTorchesOnFire`))
    (:`  `
      (`/Engine/EditorBlueprintResources/StandardMacros.CompareInt` _result (`self.NumTorchesNeeded`)
        (:`==`
          (`self.Activate`))))))

(event `SubtractOneTorch`
  (`/Engine/EditorBlueprintResources/StandardMacros.DecrementInt` (`self.NumTorchesOnFire`)))

(event `Activate`)

(fn `UserConstructionScript`
  (bind _donoteditthisarray_torchesneeded (`self.DoNotEditThisArray_TorchesNeeded`))
  (bind (_array_element _array_index) (`/Game/Gameplay/BPML_CustomMacros.ReverseForEachLoop` _donoteditthisarray_torchesneeded)
    (:`LoopBody`
      (`/Engine/EditorBlueprintResources/StandardMacros.IsValid` _array_element
        (:`Is Not Valid`
          (`KismetArrayLibrary.Array_Remove` _donoteditthisarray_torchesneeded _array_index))))
    (:`Completed`
      (`KismetSystemLibrary.FlushPersistentDebugLines`)
      (for _array_element_2 (`self.DoNotEditThisArray_TorchesNeeded`)
        (`KismetSystemLibrary.DrawDebugLine` (+ (`self.K2_GetActorLocation`) (0.0 0.0 64.0)) (+ (`self.K2_GetActorLocation` _array_element_2) (0.0 0.0 64.0)) (struct :`G` 1.0 :`B` 1.0 :`A` 1.0) 61440.0 2.8))
      (set `self.NumTorchesNeeded` (`KismetArrayLibrary.Array_Length` (`self.DoNotEditThisArray_TorchesNeeded`))))))