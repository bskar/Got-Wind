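; BP_MeltingIceWall is an ice wall that melts in steps when struck by regular or special torch dragonballs.
; Each valid impact resumes a timeline shrinking the mesh's Z scale from its construction-time value.
; A retriggerable delay pauses it after six seconds divided by the required shot count, so progress accumulates across hits.
; When the timeline finishes, the wall releases any enclosed Windstone's power and destroys itself.
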(event `self.ReceiveBeginPlay`
  (`/Engine/EditorBlueprintResources/StandardMacros.IsValid` (`self.Windstone`)
    (:`Is Not Valid`
      (set `self.HasWindstoneInside` false))))

(event `self.ReceiveActorBeginOverlap`
  (params (OtherActor :type "Actor Object Reference"))
  (bind _asbp_torch_dragonball (cast `/Game/Gameplay/Projectiles/BP_TorchDragonball` OtherActor)
    (:`then`
      (if (`/Game/Gameplay/Projectiles/BP_ProjectileBase.CanImpact` _asbp_torch_dragonball)
        (`/Game/Gameplay/Projectiles/BP_ProjectileBase.Impact` _asbp_torch_dragonball)
        (`|ExecutionSequence` :!label _label
          (:`then_0`
            (bind (_direction _scaledowntrack) (`Timeline|ScaleDownGraph` :!label _label_2)
              (:`Update`
                (`SceneComponent.SetRelativeScale3D` (`self.SM_IceWall_01`) (`KismetMathLibrary.MakeVector` 1.0 1.0 (`KismetMathLibrary.Lerp` (`self.DefaultZ_Scale`) 0.001 _scaledowntrack))))
              (:`Finished`
                (if (`self.HasWindstoneInside`)
                  (`/Game/Gameplay/BP_Windstone.ReleasePower` (`self.Windstone`)))
                (`self.K2_DestroyActor`))))
          (:`then_1`
            (`KismetSystemLibrary.RetriggerableDelay` (/ 6.0 (`KismetMathLibrary.Conv_IntToDouble` (`self.NumShotsNeeded`))))
            (goto _label_2 :!via `Stop`)))))
    (:`CastFailed`
      (bind _asbp_torch_dragonball_special (cast `/Game/Gameplay/Projectiles/BP_TorchDragonballSpecial` OtherActor))
      (if (`/Game/Gameplay/Projectiles/BP_ProjectileBase.CanImpact` _asbp_torch_dragonball_special)
        (`/Game/Gameplay/Projectiles/BP_ProjectileBase.Impact` _asbp_torch_dragonball_special)
        (goto _label)))))

(fn `UserConstructionScript`
  (set `self.DefaultZ_Scale` (.z (`SceneComponent.RelativeScale3D` (`self.SM_IceWall_01`)))))