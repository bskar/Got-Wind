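; BP_TreeBurn is a puzzle tree that burns away once enough torches are lit.
; External calls to AddOneTorch and SubtractOneTorch track a lit-torch count, and reaching NumberOfTorchesNeeded fires a one-time burn.
; The burn activates the TreeFire effect while a timeline rescales the Tree uniformly.
; The fire deactivates after a short delay, and the actor destroys itself shortly after the timeline ends.
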(event `self.ReceiveBeginPlay`
  (`ActorComponent.SetActive` (`self.TreeFire`) false false))

(event `AddOneTorch`
  (bind _result (`/Engine/EditorBlueprintResources/StandardMacros.IncrementInt` (`self.NumberOfTorchesOnFire`))
    (:`  `
      (`/Engine/EditorBlueprintResources/StandardMacros.CompareInt` _result (`self.NumberOfTorchesNeeded`)
        (:`==`
          (`/Engine/EditorBlueprintResources/StandardMacros.DoOnce` false
            (:`Completed`
              (`ActorComponent.Activate` (`self.TreeFire`) false)
              (`|ExecutionSequence`
                (:`then_0`
                  (bind (_direction _newtrack_0) (`Timeline|Timeline_0` :!via `PlayFromStart`)
                    (:`Update`
                      (`SceneComponent.SetRelativeScale3D` (`self.Tree`) (`KismetMathLibrary.MakeVector` _newtrack_0 _newtrack_0 _newtrack_0)))
                    (:`Finished`
                      (`KismetSystemLibrary.Delay` 2.8)
                      (`self.K2_DestroyActor`))))
                (:`then_1`
                  (`KismetSystemLibrary.Delay` 2.8)
                  (`ActorComponent.Deactivate` (`self.TreeFire`)))))))))))

(event `SubtractOneTorch`
  (`/Engine/EditorBlueprintResources/StandardMacros.DecrementInt` (`self.NumberOfTorchesOnFire`)))

(fn `UserConstructionScript`)