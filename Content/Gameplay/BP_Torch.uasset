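; BP_Torch is a lightable torch that reports lit and extinguished changes to an optional linked TreeToBurn.
; LightOnFire and ExtinguishFire toggle the fire effect and IsLit, adjusting the tree's torch count.
; When lit, overlap by a BP_TestWeapon with CanSpreadFire clears that flag and spawns a BP_TorchFireball at the flame, using the player's rotation.
; The construction script draws a long-duration debug circle around TorchFireTrigger.
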(event `self.ReceiveBeginPlay`
  (`ActorComponent.SetActive` (`self.TorchFireEffect`) (`self.IsLit`) false))

(event `LightOnFire`
  (if (not (`self.IsLit`))
    (`ActorComponent.Activate` (`self.TorchFireEffect`) false)
    (set `self.IsLit` true)
    (`/Engine/EditorBlueprintResources/StandardMacros.IsValid` (`self.TreeToBurn`)
      (:`Is Valid`
        (`/Game/Gameplay/BP_BurningTree.AddOneTorch` (`self.TreeToBurn`))))))

(event `self.ReceiveActorBeginOverlap`
  (params (OtherActor :type "Actor Object Reference"))
  (if (`self.IsLit`)
    (bind _asbp_test_weapon (cast `/Game/Weapons/BP_TestWeapon` OtherActor))
    (if (`/Game/Weapons/BP_TestWeapon.CanSpreadFire` _asbp_test_weapon)
      (set `/Game/Weapons/BP_TestWeapon.CanSpreadFire` false _asbp_test_weapon)
      (`|SpawnActorFromClass` "/Game/Gameplay/BP_TorchFireball.BP_TorchFireball_C" (`KismetMathLibrary.MakeTransform` (`SceneComponent.K2_GetComponentLocation` (`self.TorchFireEffect`)) (`self.K2_GetActorRotation` (`GameplayStatics.GetPlayerCharacter` 0))) "Undefined" "OverrideRootScale"))))

(event `ExtinguishFire`
  (if (`self.IsLit`)
    (`ActorComponent.Deactivate` (`self.TorchFireEffect`))
    (set `self.IsLit` false)
    (`/Engine/EditorBlueprintResources/StandardMacros.IsValid` (`self.TreeToBurn`)
      (:`Is Valid`
        (`/Game/Gameplay/BP_BurningTree.SubtractOneTorch` (`self.TreeToBurn`))))))

(fn `UserConstructionScript`
  (`KismetSystemLibrary.FlushPersistentDebugLines`)
  (`KismetSystemLibrary.DrawDebugCircle` (`SceneComponent.K2_GetComponentLocation` (`self.TorchFireTrigger`)) 593.0 64 (struct :`R` 1.0 :`A` 1.0) 61440.0 2.8 (0.0 1.0 0.0) (1.0 0.0 0.0)))