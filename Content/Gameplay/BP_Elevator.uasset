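; Elevator that rises when an overlapping BP_WindSlash turns its wheel, then sinks back to its starting height.
; Each slash counts once and restarts the UpGraph timeline, interrupting any descent unless the lift is at the top.
; Timelines drive both platform movement and wheel spin, with descent starting when the push ends or after a short pause at the top.
; The construction script sets travel limits from MaxHeight and previews them with debug lines.
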(event `self.ReceiveActorBeginOverlap`
  (params (OtherActor :type "Actor Object Reference"))
  (bind _asbp_wind_slash (cast `/Game/Weapons/BP_WindSlash` OtherActor))
  (if (`/Game/Weapons/BP_WindSlash.CanTurnWheel` _asbp_wind_slash)
    (set `/Game/Weapons/BP_WindSlash.CanTurnWheel` false _asbp_wind_slash)
    (if (`self.IsAtTheTop`)
      _
      (elif (`self.IsMovingUp`)
        (bind (_direction _uptrack) (`Timeline|UpGraph` :!via `PlayFromStart` :!label _label)
          (:`Update`
            (bind _returnvalue (`KismetMathLibrary.Lerp` 8.0 0.5 _uptrack))
            (bind _output_get (set `self.CurrentPosition` (`KismetMathLibrary.FClamp` (+ (`self.CurrentPosition`) _returnvalue) (`self.BottomPosition`) (`self.TopPosition`))))
            (if (< _output_get (`self.TopPosition`))
              (`SceneComponent.K2_AddLocalRotation` (`self.Wheel`) (`KismetMathLibrary.MakeRotator` _returnvalue) false false)
              (`self.K2_AddActorLocalOffset` (`KismetMathLibrary.MakeVector` 0.0 0.0 _returnvalue))
              (else
                (`self.StopGoingUp`)
                (`self.K2_SetActorLocation` (`KismetMathLibrary.MakeVector` (.x (`self.K2_GetActorLocation`)) (.y (`self.K2_GetActorLocation`)) (`self.TopPosition`)))
                (set `self.IsAtTheTop` true)
                (set `self.IsMovingUp` false)
                (`KismetSystemLibrary.Delay` 1.1)
                (set `self.IsAtTheTop` false)
                (set `self.IsMovingDown` true)
                (`self.GoDown`))))
          (:`Finished`
            (if (not (`self.IsAtTheTop`))
              (set `self.IsMovingUp` false)
              (set `self.IsMovingDown` true)
              (`self.GoDown`))))
        (else
          (set `self.IsMovingDown` false)
          (`self.StopGoingDown`)
          (set `self.IsMovingUp` true)
          (goto _label :!via `PlayFromStart`))))))

(event `StopGoingUp`
  (goto _label :!via `Stop`))

(event `GoDown`
  (bind (_direction _downtrack) (`Timeline|DownGraph` :!via `PlayFromStart` :!label _label_2)
    (:`Update`
      (bind _returnvalue (* _downtrack (`self.DownSpeed`)))
      (bind _output_get (set `self.CurrentPosition` (`KismetMathLibrary.FClamp` (+ (`self.CurrentPosition`) _returnvalue) (`self.BottomPosition`) (`self.TopPosition`))))
      (if (> _output_get (`self.BottomPosition`))
        (`SceneComponent.K2_AddLocalRotation` (`self.Wheel`) (`KismetMathLibrary.MakeRotator` _returnvalue) false false)
        (`self.K2_AddActorLocalOffset` (`KismetMathLibrary.MakeVector` 0.0 0.0 _returnvalue))
        (else
          (`self.K2_SetActorLocation` (`KismetMathLibrary.MakeVector` (.x (`self.K2_GetActorLocation`)) (.y (`self.K2_GetActorLocation`)) (`self.BottomPosition`)))
          (set `self.IsMovingDown` false)
          (`self.StopGoingDown`))))))

(event `StopGoingDown`
  (goto _label_2 :!via `Stop`))

(fn `UserConstructionScript`
  (bind _returnvalue (`SceneComponent.K2_GetComponentLocation` (`self.Corner4`)))
  (bind _returnvalue_2 (`SceneComponent.K2_GetComponentLocation` (`self.Corner1`)))
  (bind _returnvalue_3 (`SceneComponent.K2_GetComponentLocation` (`self.Corner2`)))
  (bind _returnvalue_4 (`SceneComponent.K2_GetComponentLocation` (`self.Corner3`)))
  (bind _output_get (set `self.CurrentPosition` (.z (`self.K2_GetActorLocation`))))
  (bind _output_get_2 (set `self.BottomPosition` _output_get))
  (bind _output_get_3 (set `self.TopPosition` (+ _output_get_2 (`self.MaxHeight`))))
  (`KismetSystemLibrary.FlushPersistentDebugLines`)
  (`KismetSystemLibrary.DrawDebugLine` _returnvalue_2 (+ _returnvalue_2 (`KismetMathLibrary.MakeVector` 0.0 0.0 (`self.MaxHeight`))) (struct :`G` 1.0 :`B` 0.000452 :`A` 1.0) 61440.0 4.2)
  (`KismetSystemLibrary.DrawDebugLine` _returnvalue_3 (+ _returnvalue_3 (`KismetMathLibrary.MakeVector` 0.0 0.0 (`self.MaxHeight`))) (struct :`G` 1.0 :`B` 0.000452 :`A` 1.0) 61440.0 4.2)
  (`KismetSystemLibrary.DrawDebugLine` _returnvalue_4 (+ _returnvalue_4 (`KismetMathLibrary.MakeVector` 0.0 0.0 (`self.MaxHeight`))) (struct :`G` 1.0 :`B` 0.000452 :`A` 1.0) 61440.0 4.2)
  (`KismetSystemLibrary.DrawDebugLine` _returnvalue (+ _returnvalue (`KismetMathLibrary.MakeVector` 0.0 0.0 (`self.MaxHeight`))) (struct :`G` 1.0 :`B` 0.000452 :`A` 1.0) 61440.0 4.2))