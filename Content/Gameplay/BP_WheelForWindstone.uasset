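; Wheel puzzle actor that spins when struck by a BP_WindSlash from one side, moving its linked Windstone up, down, left or right.
; Each valid slash restarts a timeline that eases turning speed, rolling the wheel and offsetting the stone together.
; Tracked travel is clamped to MoveDistance; reaching the end locks the wheel and calls ReleasePower on the Windstone.
; The construction script draws a debug line to the linked stone.
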(event `self.ReceiveBeginPlay`
  (set `self.MoveDistance` (`KismetMathLibrary.Abs` (`self.MoveDistance`)))
  (switch `/Game/Gameplay/E_GateType` (`self.Direction`)
    (:`NewEnumerator0`
      (bind _output_get (set `self.CurrentPosition` (.z (`self.K2_GetActorLocation` (`self.Windstone`))) :!label _label))
      (bind _output_get_2 (set `self.StartPosition` _output_get))
      (set `self.EndPosition` (+ _output_get_2 (`self.MoveDistance`))))
    (:`NewEnumerator1`
      (goto _label))
    (:`NewEnumerator2`
      (bind _output_get_3 (set `self.CurrentPosition` (.x (`self.K2_GetActorLocation` (`self.Windstone`))) :!label _label_2))
      (bind _output_get_4 (set `self.StartPosition` _output_get_3))
      (set `self.EndPosition` (+ _output_get_4 (`self.MoveDistance`))))
    (:`NewEnumerator3`
      (goto _label_2))))

(event `self.ReceiveActorBeginOverlap`
  (params (OtherActor :type "Actor Object Reference"))
  (bind _windstone (`self.Windstone`))
  (bind _asbp_wind_slash (cast `/Game/Weapons/BP_WindSlash` OtherActor))
  (if (`/Game/Weapons/BP_WindSlash.CanTurnWheel` _asbp_wind_slash)
    (set `/Game/Weapons/BP_WindSlash.CanTurnWheel` false _asbp_wind_slash)
    (if (not (`self.HasReachedEnd`))
      (if (`KismetMathLibrary.InRange_FloatFloat` (.yaw (`KismetMathLibrary.NormalizedDeltaRotator` (`self.K2_GetActorRotation`) (`self.K2_GetActorRotation` OtherActor))) 0.0 179.99999)
        (if (`self.IsTurning`)
          (bind (_direction _movetrack) (`Timeline|MoveGraph` :!via `PlayFromStart` :!label _label_3)
            (:`Update`
              (bind _returnvalue (* (`KismetMathLibrary.Lerp` (`self.TurningSpeed`) 0.5 _movetrack) (`GameplayStatics.GetWorldDeltaSeconds`) 50.0))
              (bind _output_get (set `self.CurrentPosition` (`KismetMathLibrary.FClamp` (+ (`self.CurrentPosition`) _returnvalue) (`self.StartPosition`) (`self.EndPosition`))))
              (if (< _output_get (`self.EndPosition`))
                (`SceneComponent.K2_AddLocalRotation` (`self.Wheel`) (`KismetMathLibrary.MakeRotator` _returnvalue) false false)
                (switch `/Game/Gameplay/E_GateType` (`self.Direction`)
                  (:`NewEnumerator0`
                    (`self.K2_AddActorLocalOffset` _windstone (`KismetMathLibrary.MakeVector` 0.0 0.0 _returnvalue) false false))
                  (:`NewEnumerator1`
                    (bind _returnvalue_2 (* _returnvalue -1.0))
                    (`self.K2_AddActorLocalOffset` _windstone (`KismetMathLibrary.MakeVector` 0.0 0.0 _returnvalue_2) false false))
                  (:`NewEnumerator2`
                    (`self.K2_AddActorLocalOffset` _windstone (`KismetMathLibrary.MakeVector` _returnvalue_2) false false))
                  (:`NewEnumerator3`
                    (`self.K2_AddActorLocalOffset` _windstone (`KismetMathLibrary.MakeVector` _returnvalue) false false)))
                (else
                  (`self.StopMoving`)
                  (set `self.HasReachedEnd` true)
                  (set `self.IsTurning` false)
                  (`/Game/Gameplay/BP_Windstone.ReleasePower` (`self.Windstone`)))))
            (:`Finished`
              (set `self.IsTurning` false)))
          (else
            (set `self.IsTurning` true)
            (goto _label_3 :!via `PlayFromStart`)))))))

(event `StopMoving`
  (goto _label_3 :!via `Stop`))

(fn `UserConstructionScript`
  (bind _windstone (`self.Windstone`))
  (set `self.MoveDistance` (`KismetMathLibrary.Abs` (`self.MoveDistance`)))
  (switch `/Game/Gameplay/E_GateType` (`self.Direction`)
    (:`NewEnumerator0`
      (bind _output_get (set `self.CurrentPosition` (.z (`self.K2_GetActorLocation` (`self.Windstone`))) :!label _label))
      (bind _output_get_2 (set `self.StartPosition` _output_get))
      (set `self.EndPosition` (+ _output_get_2 (`self.MoveDistance`))))
    (:`NewEnumerator1`
      (goto _label))
    (:`NewEnumerator2`
      (bind _output_get_3 (set `self.CurrentPosition` (.x (`self.K2_GetActorLocation` (`self.Windstone`))) :!label _label_2))
      (bind _output_get_4 (set `self.StartPosition` _output_get_3))
      (set `self.EndPosition` (+ _output_get_4 (`self.MoveDistance`))))
    (:`NewEnumerator3`
      (goto _label_2)))
  (`KismetSystemLibrary.FlushPersistentDebugLines`)
  (`/Engine/EditorBlueprintResources/StandardMacros.IsValid` _windstone
    (:`Is Valid`
      (`KismetSystemLibrary.DrawDebugLine` (+ (`self.K2_GetActorLocation`) (0.0 0.0 100.0)) (`self.K2_GetActorLocation` _windstone) (struct :`G` 1.0 :`B` 0.000452 :`A` 1.0) 61440.0 4.2))))