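; Checkpoint actor that sets an overlapping ThirdPersonCharacter's current respawn point to its assigned RespawnPoint, printing an error if that reference is invalid.
; When a RespawnPoint is set, the construction script flushes persistent debug lines and draws a long-lived line to it.
; It also scans all checkpoints and warns when another shares the same RespawnPoint.
; Disconnected construction logic for label text and numbered checkpoints never runs.
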(event `self.ReceiveActorBeginOverlap`
  (params (OtherActor :type "Actor Object Reference"))
  (bind _respawnpoint (`self.RespawnPoint`))
  (bind _asthird_person_character (cast `/Game/Characters/Player/ThirdPersonCharacter` OtherActor))
  (`/Engine/EditorBlueprintResources/StandardMacros.IsValid` _respawnpoint
    (:`Is Valid`
      (set `/Game/Characters/Player/ThirdPersonCharacter.CurrentRespawnPoint` _respawnpoint _asthird_person_character))
    (:`Is Not Valid`
      (`KismetSystemLibrary.PrintString` (`KismetStringLibrary.Concat_StrStr` (`KismetSystemLibrary.GetDisplayName` self) " has an invalid RespawnPoint! Please fix.") true true (struct :`G` 0.66 :`B` 1.0 :`A` 1.0) 4.2))))

(fn `UserConstructionScript`
  (bind _respawnpoint (`self.RespawnPoint`))
  (`/Engine/EditorBlueprintResources/StandardMacros.IsValid` _respawnpoint
    (:`Is Valid`
      (`KismetSystemLibrary.FlushPersistentDebugLines`)
      (`KismetSystemLibrary.DrawDebugLine` (`self.K2_GetActorLocation`) (+ (`self.K2_GetActorLocation` _respawnpoint) (0.0 0.0 72.0)) (struct :`G` 1.0 :`B` 0.000452 :`A` 1.0) 61440.0 16.0)
      (bind _outactors (`GameplayStatics.GetAllActorsOfClass` "BP_Checkpoint_C"))
      (for _array_element _outactors
        (if (and (== (`/Game/Gameplay/PlayerRespawning/BP_Checkpoint.RespawnPoint` _array_element) (`self.RespawnPoint`)) (!= _array_element self))
          (`KismetSystemLibrary.PrintString` (`KismetStringLibrary.Concat_StrStr` "Warning: " (`KismetSystemLibrary.GetDisplayName` (`self.RespawnPoint`)) " is also assigned to another Checkpoint!") true true (struct :`G` 0.66 :`B` 1.0 :`A` 1.0) 8.4))))))