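; BP_DeathPoint is a box kill volume that calls KillVayu on any BP_Vayu actor that overlaps it.
; With UseCustomRespawnPoint on, it first sets Vayu's CurrentRespawnPoint to the custom one, or only prints an error, without killing, if that is invalid.
; The construction script sizes the box from Size and draws a long-lived debug line to a valid custom respawn point.
; Text-label update logic is left unconnected.
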(event `self.ReceiveActorBeginOverlap`
  (params (OtherActor :type "Actor Object Reference"))
  (bind _customrespawnpoint (`self.CustomRespawnPoint`))
  (bind _asbp_vayu (cast `/Game/Characters/Player/BP_Vayu` OtherActor))
  (if (`self.UseCustomRespawnPoint`)
    (`/Engine/EditorBlueprintResources/StandardMacros.IsValid` _customrespawnpoint
      (:`Is Valid`
        (set `/Game/Characters/Player/BP_Vayu.CurrentRespawnPoint` _customrespawnpoint _asbp_vayu)
        (`/Game/Characters/Player/BP_Vayu.KillVayu` _asbp_vayu :!label _label))
      (:`Is Not Valid`
        (`KismetSystemLibrary.PrintString` (`KismetStringLibrary.Concat_StrStr` (`KismetSystemLibrary.GetDisplayName` self) " has an invalid RespawnPoint! Please fix.") true true (struct :`G` 0.66 :`B` 1.0 :`A` 1.0) 4.2)))
    (else
      (goto _label))))

(fn `UserConstructionScript`
  (bind _customrespawnpoint (`self.CustomRespawnPoint`))
  (`BoxComponent.SetBoxExtent` (`self.Box`) (`self.Size`) true)
  (if (`self.UseCustomRespawnPoint`)
    (`/Engine/EditorBlueprintResources/StandardMacros.IsValid` _customrespawnpoint
      (:`Is Valid`
        (`KismetSystemLibrary.FlushPersistentDebugLines`)
        (`KismetSystemLibrary.DrawDebugLine` (`self.K2_GetActorLocation`) (+ (`self.K2_GetActorLocation` _customrespawnpoint) (0.0 0.0 72.0)) (struct :`G` 1.0 :`B` 0.000452 :`A` 1.0) 61440.0 16.0)))))