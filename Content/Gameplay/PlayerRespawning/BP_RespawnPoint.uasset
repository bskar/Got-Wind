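; BP_RespawnPoint is a respawn point actor that plays a rising and falling flower animation when its RespawnSequence event fires.
; The event unhides the actor and chains two timelines, whose up and down tracks incrementally spin BigFlower in yaw and move it along local Z.
; When the second finishes, the actor hides, stops ticking, and restores the flower's relative location cached in the construction script.
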(event `RespawnSequence`
  (bind _bigflower (`self.BigFlower`))
  (bind _bigflower_2 (`self.BigFlower`))
  (`self.SetActorHiddenInGame` false)
  (`self.SetActorTickEnabled` true)
  (bind (_direction _uptrack) (`Timeline|Timeline_0` :!via `PlayFromStart`)
    (:`Update`
      (`SceneComponent.K2_AddLocalRotation` _bigflower (`KismetMathLibrary.MakeRotator` 0.0 0.0 _uptrack) false false)
      (`SceneComponent.K2_AddLocalOffset` _bigflower (`KismetMathLibrary.MakeVector` 0.0 0.0 _uptrack) false false))
    (:`Finished`
      (bind (_direction_2 _downtrack) (`Timeline|Timeline_1` :!via `PlayFromStart`)
        (:`Update`
          (`SceneComponent.K2_AddLocalRotation` _bigflower_2 (`KismetMathLibrary.MakeRotator` 0.0 0.0 _downtrack) false false)
          (`SceneComponent.K2_AddLocalOffset` _bigflower_2 (`KismetMathLibrary.MakeVector` 0.0 0.0 _downtrack) false false))
        (:`Finished`
          (`self.SetActorHiddenInGame` true)
          (`self.SetActorTickEnabled` false)
          (`SceneComponent.K2_SetRelativeLocation` (`self.BigFlower`) (`self.DefaultLocation`) false false))))))

(fn `UserConstructionScript`
  (set `self.DefaultLocation` (`SceneComponent.RelativeLocation` (`self.BigFlower`))))