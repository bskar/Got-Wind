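; BP_SymbolGate is a double gate with a spiral lock piece that plays a one-time unlock and open animation when OpenSesame is called.
; The construction script records the spiral's starting pitch as its locked rotation.
; A timeline then turns the spiral 90 degrees from that pitch on one track and swings the left and right leaves outward in opposite directions on another.
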(event `OpenSesame`
  (bind _defaultlockedrotation (`self.DefaultLockedRotation`))
  (`/Engine/EditorBlueprintResources/StandardMacros.DoOnce` false
    (:`Completed`
      (bind (_direction _unlocktrack _opentrack) (`Timeline|UnlockAndOpenGraph` :!via `PlayFromStart`)
        (:`Update`
          (`SceneComponent.K2_SetRelativeRotation` (`self.SM_GateSpiral_01`) (`KismetMathLibrary.MakeRotator` 0.0 (`KismetMathLibrary.Lerp` _defaultlockedrotation (+ _defaultlockedrotation 90.0) _unlocktrack) 180.0) false false)
          (`SceneComponent.K2_SetRelativeRotation` (`self.SM_GateLeft_01`) (`KismetMathLibrary.MakeRotator` 0.0 0.0 (`KismetMathLibrary.Lerp` 0.0 -105.0 _opentrack)) false false)
          (`SceneComponent.K2_SetRelativeRotation` (`self.SM_GateRight_01`) (`KismetMathLibrary.MakeRotator` 0.0 0.0 (`KismetMathLibrary.Lerp` 0.0 105.0 _opentrack)) false false))))))

(fn `UserConstructionScript`
  (set `self.DefaultLockedRotation` (.pitch (`SceneComponent.RelativeRotation` (`self.SM_GateSpiral_01`)))))