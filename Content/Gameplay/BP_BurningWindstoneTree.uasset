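; Burning Windstone tree actor that, when activated, burns away and advances the player's progress.
; Activate runs once, switching on the TreeFire effect while a timeline drives the tree mesh's scale for the shrink.
; TreeFire deactivates after a short delay; once the timeline finishes and a further delay passes, it sets Progress on the ThirdPersonCharacter and destroys itself.
; Torch counting events defer to the parent class.
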(event `self.ReceiveBeginPlay`
  (`parent.ReceiveBeginPlay`)
  (`ActorComponent.SetActive` (`self.TreeFire`) false false))

(event `self.AddOneTorch`
  (`parent.AddOneTorch`))

(event `self.SubtractOneTorch`
  (`parent.SubtractOneTorch`))

(event `self.Activate`
  (`/Engine/EditorBlueprintResources/StandardMacros.DoOnce` false
    (:`Completed`
      (`ActorComponent.Activate` (`self.TreeFire`) false)
      (`|ExecutionSequence`
        (:`then_0`
          (bind (_direction _scaledowntrack) (`Timeline|ScaleDownGraph` :!via `PlayFromStart`)
            (:`Update`
              (`SceneComponent.SetRelativeScale3D` (`self.Tree`) (`KismetMathLibrary.VLerp` (0.0 0.0 0.0) (1.0 1.0 1.0) _scaledowntrack)))
            (:`Finished`
              (`KismetSystemLibrary.Delay` 2.8)
              (set `/Game/Characters/Player/ThirdPersonCharacter.Progress` (`self.ProgressToSet`) (cast `/Game/Characters/Player/ThirdPersonCharacter` (`GameplayStatics.GetPlayerCharacter` 0) :!pure true))
              (`self.K2_DestroyActor`))))
        (:`then_1`
          (`KismetSystemLibrary.Delay` 2.8)
          (`ActorComponent.Deactivate` (`self.TreeFire`)))))))

(fn `UserConstructionScript`
  (`parent.UserConstructionScript`))