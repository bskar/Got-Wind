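; BP_SpinnyPlatform is an interactive platform that takes player input while a ThirdPersonCharacter overlaps it.
; Overlap begin and end enable and disable input from player controller 0.
; Pressing I activates the SpinnyPlatformEffect component and plays a timeline, with a DoOnce blocking retriggers until it finishes.
; A local yaw rotation driven by the timeline's SpinTrack exists but is unconnected, so this graph never spins the platform.
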(event `self.ReceiveActorBeginOverlap`
  (params (OtherActor :type "Actor Object Reference"))
  (cast `/Game/Dev/ThirdPersonBP/Blueprints/ThirdPersonCharacter` OtherActor)
  (`self.EnableInput` (`GameplayStatics.GetPlayerController` 0)))

(event `self.ReceiveActorEndOverlap`
  (params (OtherActor :type "Actor Object Reference"))
  (cast `/Game/Dev/ThirdPersonBP/Blueprints/ThirdPersonCharacter` OtherActor)
  (`self.DisableInput` (`GameplayStatics.GetPlayerController` 0)))

(event `Key|I`
  (params (Key :type "Key Structure" :default "AnyKey"))
  (:`Pressed`
    (`/Engine/EditorBlueprintResources/StandardMacros.DoOnce` false :!label _label
      (:`Completed`
        (`ActorComponent.Activate` (`self.SpinnyPlatformEffect`) false)
        (bind (_direction _spintrack) (`Timeline|Timeline_0` :!via `PlayFromStart`)
          (:`Finished`
            (goto _label :!via `Reset`)))))))

(fn `UserConstructionScript`)