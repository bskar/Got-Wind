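; BP_DeathPoint is a hazard actor that kills the player character on overlap and sets where it respawns.
; On overlap it assigns its RespawnPoint as the ThirdPersonCharacter's CurrentRespawnPoint, then calls KillVayu, or prints an error if the point is invalid.
; The construction script labels the actor with the respawn point's name, or NONE, and adjusts the text scale to offset non-uniform Y/Z root scaling.
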(event `self.ReceiveActorBeginOverlap`
  (params (OtherActor :type "Actor Object Reference"))
  (bind _respawnpoint (`self.RespawnPoint`))
  (bind _asthird_person_character (cast `/Game/Characters/Player/ThirdPersonCharacter` OtherActor))
  (`/Engine/EditorBlueprintResources/StandardMacros.IsValid` _respawnpoint
    (:`Is Valid`
      (set `/Game/Characters/Player/ThirdPersonCharacter.CurrentRespawnPoint` _respawnpoint _asthird_person_character)
      (`/Game/Characters/Player/ThirdPersonCharacter.KillVayu` _asthird_person_character))
    (:`Is Not Valid`
      (`KismetSystemLibrary.PrintString` (`KismetStringLibrary.Concat_StrStr` (`KismetSystemLibrary.GetDisplayName` self) " has an invalid RespawnPoint! Please fix.") true true (struct :`G` 0.66 :`B` 1.0 :`A` 1.0) 4.2))))

(fn `UserConstructionScript`
  (bind _respawnpointtext (`self.RespawnPointText`))
  (bind _y (.y (`SceneComponent.K2_GetComponentScale` (`self.DefaultSceneRoot`))))
  (bind _z (.z (`SceneComponent.K2_GetComponentScale` (`self.DefaultSceneRoot`))))
  (`/Engine/EditorBlueprintResources/StandardMacros.IsValid` (`self.RespawnPoint`)
    (:`Is Valid`
      (`TextRenderComponent.K2_SetText` _respawnpointtext (`KismetTextLibrary.Conv_StringToText` (`KismetSystemLibrary.GetDisplayName` (`self.RespawnPoint`)))))
    (:`Is Not Valid`
      (`TextRenderComponent.K2_SetText` (`self.RespawnPointText`) (`KismetTextLibrary.Conv_StringToText` "NONE"))))
  (if (>= _y _z)
    (`TextRenderComponent.SetYScale` _respawnpointtext (/ _y _z))
    (else
      (`TextRenderComponent.SetXScale` _respawnpointtext (/ _z _y)))))