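; Base torch actor whose TorchType selects behavior: fire spreading, timed or one-shot burn, activation counting, or dragon variants with empty hook events.
; When a BP_WindSlash able to spread fire overlaps certain lit torches, they launch a fireball along the player's facing.
; Lighting and extinguishing toggle the particle and notify assigned GuardianImps.
; The construction script syncs those imps' watch lists and optionally draws the fireball's reach as a debug circle.
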(event `self.ReceiveBeginPlay`
  (bind _guardianimps (`self.GuardianImps`))
  (bind _torchfire (`self.TorchFire`))
  (switch `/Game/Gameplay/Torches/E_TorchType` (`self.TorchType`)
    (:`NewEnumerator2`
      (bind (_array_element _array_index) (`/Game/Gameplay/BPML_CustomMacros.ReverseForEachLoop` _guardianimps :!label _label)
        (:`LoopBody`
          (`/Engine/EditorBlueprintResources/StandardMacros.IsValid` _array_element
            (:`Is Not Valid`
              (`KismetArrayLibrary.Array_Remove` (`self.GuardianImps`) _array_index))))
        (:`Completed`
          (if (`self.IsLit`)
            (switch `/Game/Gameplay/Torches/E_TorchType` (`self.TorchType`)
              (:`NewEnumerator2`
                _)
              (:`NewEnumerator1`
                _)
              (:`NewEnumerator0`
                _)
              (:`NewEnumerator3`
                (`KismetSystemLibrary.K2_SetTimer` self "ExtinguishFire" (`self.TimedFireDuration`)))
              (:`NewEnumerator4`
                _)
              (:`NewEnumerator5`
                _))
            ;[1 1 1] Important!
            (`self.ThisTorchIsOn`)
            (switch `/Game/Gameplay/Torches/E_TorchType` (`self.TorchType`)
              (:`NewEnumerator0`
                (`self.AddOne`)))
            (else
              (`ActorComponent.Deactivate` _torchfire)
              (`ParticleSystemComponent.SetTemplate` _torchfire null))))))
    (:`NewEnumerator1`
      (goto _label))
    (:`NewEnumerator0`
      (goto _label))
    (:`NewEnumerator3`
      (goto _label))
    (:`NewEnumerator4`
      (goto _label))
    (:`NewEnumerator5`
      (goto _label))
    (:`NewEnumerator6`
      (`KismetArrayLibrary.Array_Clear` _guardianimps :!label _label_2))
    (:`NewEnumerator7`
      (goto _label_2))))

(event `self.ReceiveActorBeginOverlap`
  (params (OtherActor :type "Actor Object Reference"))
  (bind _returnvalue (`KismetMathLibrary.MakeTransform` (`SceneComponent.K2_GetComponentLocation` (`self.TorchTrigger`)) (`self.K2_GetActorRotation` (`GameplayStatics.GetPlayerCharacter` 0))))
  (switch `/Game/Gameplay/Torches/E_TorchType` (`self.TorchType`)
    (:`NewEnumerator2`
      _)
    (:`NewEnumerator1`
      _)
    (:`NewEnumerator3`
      _)
    (:`NewEnumerator4`
      _)
    (:`NewEnumerator5`
      _))
  (if (`self.IsLit`)
    (bind _asbp_wind_slash (cast `/Game/Weapons/BP_WindSlash` OtherActor))
    (if (`/Game/Weapons/BP_WindSlash.CanSpreadFire` _asbp_wind_slash)
      (set `/Game/Weapons/BP_WindSlash.CanSpreadFire` false _asbp_wind_slash)
      (switch `/Game/Gameplay/Torches/E_TorchType` (`self.TorchType`)
        (:`NewEnumerator2`
          (`|SpawnActorFromClass` "/Game/Gameplay/Projectiles/BP_TorchFireball.BP_TorchFireball_C" _returnvalue "Undefined" "OverrideRootScale" :!label _label_3)
          (switch `/Game/Gameplay/Torches/E_TorchType` (`self.TorchType`)
            (:`NewEnumerator5`
              (`self.ExtinguishFire`))))
        (:`NewEnumerator1`
          (goto _label_3))
        (:`NewEnumerator3`
          (goto _label_3))
        (:`NewEnumerator4`
          (`|SpawnActorFromClass` "/Game/Gameplay/Projectiles/BP_TorchFireballLongRange.BP_TorchFireballLongRange_C" _returnvalue "Undefined" "OverrideRootScale"))
        (:`NewEnumerator5`
          (goto _label_3))))))

(event `LightOnFire`
  (bind _torchfire (`self.TorchFire`))
  (if (`self.IsLit`)
    (switch `/Game/Gameplay/Torches/E_TorchType` (`self.TorchType`)
      (:`NewEnumerator3`
        (`KismetSystemLibrary.K2_SetTimer` self "ExtinguishFire" (`self.TimedFireDuration`))))
    (else
      (switch `/Game/Gameplay/Torches/E_TorchType` (`self.TorchType`)
        (:`NewEnumerator2`
          (`ParticleSystemComponent.SetTemplate` _torchfire "/Game/InfinityBladeEffects/Effects/FX_Combat_Base/WeaponShimmer/Fire/P_WeaponShimmer_Fire_Blunt.P_WeaponShimmer_Fire_Blunt" :!label _label_4)
          (`ActorComponent.Activate` _torchfire false)
          (set `self.IsLit` true)
          (`self.ThisTorchIsOn`)
          (switch `/Game/Gameplay/Torches/E_TorchType` (`self.TorchType`)
            (:`NewEnumerator0`
              (`self.AddOne`))
            (:`NewEnumerator3`
              (`KismetSystemLibrary.K2_SetTimer` self "ExtinguishFire" (`self.TimedFireDuration`)))))
        (:`NewEnumerator1`
          (goto _label_4))
        (:`NewEnumerator0`
          (goto _label_4))
        (:`NewEnumerator3`
          (goto _label_4))
        (:`NewEnumerator4`
          (goto _label_4))
        (:`NewEnumerator5`
          (goto _label_4))
        (:`NewEnumerator6`
          (set `self.IsLit` true :!label _label_5)
          (`self.DragonDown`))
        (:`NewEnumerator7`
          (goto _label_5))))))

(event `ExtinguishFire`
  (bind _torchfire (`self.TorchFire`))
  (if (`self.IsLit`)
    (switch `/Game/Gameplay/Torches/E_TorchType` (`self.TorchType`)
      (:`NewEnumerator2`
        _)
      (:`NewEnumerator1`
        _)
      (:`NewEnumerator0`
        _)
      (:`NewEnumerator3`
        _)
      (:`NewEnumerator4`
        _)
      (:`NewEnumerator5`
        _))
    (`ActorComponent.Deactivate` _torchfire)
    (`ParticleSystemComponent.SetTemplate` _torchfire null)
    (set `self.IsLit` false)
    (`self.ThisTorchIsOff`)
    (switch `/Game/Gameplay/Torches/E_TorchType` (`self.TorchType`)
      (:`NewEnumerator0`
        (`self.SubtractOne`)))))

(event `ThisTorchIsOn`
  (bind _guardianimps (`self.GuardianImps`))
  (switch `/Game/Gameplay/Torches/E_TorchType` (`self.TorchType`)
    (:`NewEnumerator2`
      _)
    (:`NewEnumerator1`
      _)
    (:`NewEnumerator0`
      _)
    (:`NewEnumerator3`
      _)
    (:`NewEnumerator4`
      _)
    (:`NewEnumerator5`
      _))
  (if (!= (`KismetArrayLibrary.Array_Length` _guardianimps) 0)
    (bind (_array_element _array_index) (`/Game/Gameplay/BPML_CustomMacros.ReverseForEachLoop` _guardianimps)
      (:`LoopBody`
        (`/Engine/EditorBlueprintResources/StandardMacros.IsValid` _array_element
          (:`Is Valid`
            (`/Game/Characters/NPC/Imp/BP_Imp.TorchNeedsHelp` _array_element self))
          (:`Is Not Valid`
            (`KismetArrayLibrary.Array_Remove` (`self.GuardianImps`) _array_index)))))))

(event `ThisTorchIsOff`
  (bind _guardianimps (`self.GuardianImps`))
  (switch `/Game/Gameplay/Torches/E_TorchType` (`self.TorchType`)
    (:`NewEnumerator2`
      _)
    (:`NewEnumerator1`
      _)
    (:`NewEnumerator0`
      _)
    (:`NewEnumerator3`
      _)
    (:`NewEnumerator4`
      _)
    (:`NewEnumerator5`
      _))
  (if (!= (`KismetArrayLibrary.Array_Length` _guardianimps) 0)
    (bind (_array_element _array_index) (`/Game/Gameplay/BPML_CustomMacros.ReverseForEachLoop` _guardianimps)
      (:`LoopBody`
        (`/Engine/EditorBlueprintResources/StandardMacros.IsValid` _array_element
          (:`Is Valid`
            (`/Game/Characters/NPC/Imp/BP_Imp.TorchIsOkay` _array_element self))
          (:`Is Not Valid`
            (`KismetArrayLibrary.Array_Remove` (`self.GuardianImps`) _array_index)))))))

(event `AddOne`)

(event `SubtractOne`)

(event `DragonDown`)

(event `DragonFire`)

(event `DragonUp`)

(fn `UserConstructionScript`
  (switch `/Game/Gameplay/Torches/E_TorchType` (`self.TorchType`)
    (:`NewEnumerator2`
      _)
    (:`NewEnumerator1`
      _)
    (:`NewEnumerator0`
      _)
    (:`NewEnumerator3`
      _)
    (:`NewEnumerator4`
      _)
    (:`NewEnumerator5`
      _)
    (:`NewEnumerator6`
      _)
    (:`NewEnumerator7`
      _))
  (`PrimitiveComponent.SetWalkableSlopeOverride` (`self.Torch`) (make `WalkableSlopeOverride` "WalkableSlope_Unwalkable" 0.0))
  (if (`self.HasDebugFireballRadius`)
    (`KismetSystemLibrary.FlushPersistentDebugLines`)
    (`KismetSystemLibrary.DrawDebugCircle` (`SceneComponent.K2_GetComponentLocation` (`self.TorchTrigger`)) (+ (* (`self.FireballInitialSpeed`) (`self.FireballActiveSeconds`)) (`self.FireballTriggerRadius`) (`SphereComponent.SphereRadius` (`self.TorchTrigger`))) 256 (`self.DebugLineColor`) 61440.0 2.8 (0.0 1.0 0.0) (1.0 0.0 0.0) true))
  (if (!= (`KismetArrayLibrary.Array_Length` (`self.GuardianImps`)) 0)
    (for _array_element (`self.GuardianImps`)
      (`/Engine/EditorBlueprintResources/StandardMacros.IsValid` _array_element
        (:`Is Valid`
          (`KismetArrayLibrary.Array_AddUnique` (`/Game/Characters/NPC/Imp/BP_Imp.DoNotEditThisArray_TorchesToWatch` _array_element) self)))))
  (bind _outactors (`GameplayStatics.GetAllActorsOfClass` "/Game/Characters/NPC/Imp/BP_Imp.BP_Imp_C"))
  (bind _array_element_2 (`/Game/Gameplay/BPML_CustomMacros.ReverseForEachLoop` _outactors)
    (:`LoopBody`
      (bind _donoteditthisarray_torchestowatch (`/Game/Characters/NPC/Imp/BP_Imp.DoNotEditThisArray_TorchesToWatch` _array_element_2))
      (if (and (`KismetArrayLibrary.Array_Contains` _donoteditthisarray_torchestowatch self) (not (`KismetArrayLibrary.Array_Contains` (`self.GuardianImps`) _array_element_2)))
        (`KismetArrayLibrary.Array_RemoveItem` _donoteditthisarray_torchestowatch self)
        (`KismetSystemLibrary.PrintString` "IF THIS TEXT APPEARED WHEN YOU OPENED THE PROJECT, TELL BO!" true true (struct :`G` 0.66 :`B` 1.0 :`A` 1.0) 42.0)))))