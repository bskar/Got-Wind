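; Torch variant shaped as a dragon head that lowers into a firing pose and shoots a BP_TorchDragonballSpecial.
; Chained timelines burn down the tongue, move the teeth and rotate the head until ready to fire.
; DragonFire spawns the projectile, then timelines reset the parts, raise the head and clear IsLit.
; Construction script disables the inherited torch visuals, derives rotation limits and draws a debug line showing fireball reach.
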(event `self.ReceiveBeginPlay`
  (bind _dragonsparks (`self.DragonSparks`))
  (`parent.ReceiveBeginPlay`)
  (if (`self.IsLit`)
    (`self.DragonDown`)
    (else
      (`ActorComponent.Deactivate` _dragonsparks)
      (`ParticleSystemComponent.SetTemplate` _dragonsparks null))))

(event `self.ReceiveActorBeginOverlap`
  (params (OtherActor :type "Actor Object Reference")))

(event `self.LightOnFire`
  (`parent.LightOnFire`))

(event `self.DragonDown`
  (bind _dragonsparks (`self.DragonSparks`))
  (`ParticleSystemComponent.SetTemplate` _dragonsparks "/Game/SimpleCartoonFX/FX/Muzzle_DragonFuse.Muzzle_DragonFuse")
  (`ActorComponent.Activate` _dragonsparks false)
  (bind (_direction _tonguedowntrack _teethuptrack) (`Timeline|BurningGraph` :!via `PlayFromStart`)
    (:`Update`
      (`SceneComponent.SetRelativeScale3D` (`self.DragonTongue`) (`KismetMathLibrary.MakeVector` 1.0 1.0 (`KismetMathLibrary.Lerp` 1.0 0.3 _tonguedowntrack)))
      (`SceneComponent.K2_SetRelativeLocation` (`self.DragonTeeth`) (`KismetMathLibrary.MakeVector` 0.0 0.0 (`KismetMathLibrary.Lerp` -33.0 -18.0 _teethuptrack)) false false))
    (:`Finished`
      (bind (_direction_2 _downtrack) (`Timeline|DownGraph` :!via `PlayFromStart` :!label _label)
        (:`Update`
          (bind _returnvalue (`KismetMathLibrary.Lerp` 0.0 24.0 _downtrack))
          (bind _output_get (set `self.CurrentRotation` (`KismetMathLibrary.FClamp` (+ (`self.CurrentRotation`) _returnvalue) (`self.DefaultRotation`) (`self.ShootingRotation`))))
          (if (< _output_get (`self.ShootingRotation`))
            (`SceneComponent.K2_AddRelativeRotation` (`self.DragonHead`) (`KismetMathLibrary.MakeRotator` _returnvalue) false false)
            (else
              (`SceneComponent.K2_SetRelativeRotation` (`self.DragonHead`) (`KismetMathLibrary.MakeRotator` (`self.ShootingRotation`) (.pitch (`SceneComponent.RelativeRotation` (`self.DragonHead`))) (.yaw (`SceneComponent.RelativeRotation` (`self.DragonHead`)))) false false)
              (`self.StopDragonDown`)
              (set `self.IsReadyToFire` true))))))))

(event `StopDragonDown`
  (goto _label :!via `Stop`))

(event `self.DragonFire`
  (bind _dragonsparks (`self.DragonSparks`))
  (set `self.IsReadyToFire` false)
  (`|SpawnActorFromClass` "/Game/Gameplay/Projectiles/BP_TorchDragonballSpecial.BP_TorchDragonballSpecial_C" (`SceneComponent.K2_GetComponentToWorld` (`self.DragonballSpawnTransform`)) "Undefined" "OverrideRootScale")
  (`ActorComponent.Deactivate` _dragonsparks)
  (`ParticleSystemComponent.SetTemplate` _dragonsparks null)
  (`KismetSystemLibrary.Delay` 0.21)
  (bind (_direction _tongueuptrack _teethdowntrack) (`Timeline|ResettingGraph` :!via `PlayFromStart`)
    (:`Update`
      (`SceneComponent.SetRelativeScale3D` (`self.DragonTongue`) (`KismetMathLibrary.MakeVector` 1.0 1.0 (`KismetMathLibrary.Lerp` 0.3 1.0 _tongueuptrack)))
      (`SceneComponent.K2_SetRelativeLocation` (`self.DragonTeeth`) (`KismetMathLibrary.MakeVector` 0.0 0.0 (`KismetMathLibrary.Lerp` -18.0 -33.0 _teethdowntrack)) false false))
    (:`StartGoingUp`
      (`self.DragonUp`))))

(event `self.DragonUp`
  (bind (_direction _uptrack) (`Timeline|UpGraph` :!via `PlayFromStart` :!label _label_2)
    (:`Update`
      (bind _returnvalue (`KismetMathLibrary.Lerp` 0.0 -22.0 _uptrack))
      (bind _output_get (set `self.CurrentRotation` (`KismetMathLibrary.FClamp` (+ (`self.CurrentRotation`) _returnvalue) (`self.DefaultRotation`) (`self.ShootingRotation`))))
      (if (> _output_get (`self.DefaultRotation`))
        (`SceneComponent.K2_AddRelativeRotation` (`self.DragonHead`) (`KismetMathLibrary.MakeRotator` _returnvalue) false false)
        (else
          (`SceneComponent.K2_SetRelativeRotation` (`self.DragonHead`) (`KismetMathLibrary.MakeRotator` (`self.DefaultRotation`) (.pitch (`SceneComponent.RelativeRotation` (`self.DragonHead`))) (.yaw (`SceneComponent.RelativeRotation` (`self.DragonHead`)))) false false)
          (`self.StopDragonUp`)
          (set `self.IsLit` false))))))

(event `StopDragonUp`
  (goto _label_2 :!via `Stop`))

(fn `UserConstructionScript`
  (bind _torch (`self.Torch`))
  (bind _returnvalue (`SceneComponent.K2_GetComponentLocation` (`self.DragonballSpawnTransform`)))
  (bind _returnvalue_2 (+ (* (`self.FireballInitialSpeed`) (`self.FireballActiveSeconds`)) (`self.FireballTriggerRadius`) (`SphereComponent.SphereRadius` (`self.TorchTrigger`))))
  (`parent.UserConstructionScript`)
  (bind _output_get (set `self.CurrentRotation` (.roll (`SceneComponent.RelativeRotation` (`self.DragonHead`)))))
  (bind _output_get_2 (set `self.DefaultRotation` _output_get))
  (set `self.ShootingRotation` (+ _output_get_2 (`self.MaxRotation`)))
  (`ActorComponent.Deactivate` _torch)
  (`ActorComponent.Deactivate` (`self.TorchFire`))
  (`PrimitiveComponent.SetCollisionEnabled` _torch "NoCollision")
  (`PrimitiveComponent.SetCollisionEnabled` (`self.TorchFire`) "NoCollision")
  (`SceneComponent.SetHiddenInGame` _torch true true)
  (`SceneComponent.SetHiddenInGame` (`self.TorchFire`) true true)
  (`ActorComponent.SetComponentTickEnabled` _torch false)
  (`ActorComponent.SetComponentTickEnabled` (`self.TorchFire`) false)
  (`KismetSystemLibrary.FlushPersistentDebugLines`)
  (`KismetSystemLibrary.DrawDebugLine` _returnvalue (`KismetMathLibrary.MakeVector` (+ (* (.x (`self.GetActorRightVector`)) _returnvalue_2) (.x _returnvalue)) (+ (* (.y (`self.GetActorRightVector`)) _returnvalue_2) (.y _returnvalue)) (.z _returnvalue)) (`self.DebugLineColor`) 61440.0 3.4))