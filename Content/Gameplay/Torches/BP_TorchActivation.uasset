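; Torch child Blueprint that counts toward activating linked torch-activated objects and spin pads.
; AddOne and SubtractOne forward count changes to every valid linked target, while BeginPlay prunes invalid links.
; The Construction Script registers the torch on its targets, removes it from unlinked ones and recomputes each target's required torch count.
; Overlap, extinguish and on/off overrides are empty, leaving their parent calls disconnected.
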(event `self.ReceiveBeginPlay`
  (bind _activationobjects (`self.ActivationObjects`))
  (bind _activationpads (`self.ActivationPads`))
  (`parent.ReceiveBeginPlay`)
  (bind (_array_element _array_index) (`/Game/Gameplay/BPML_CustomMacros.ReverseForEachLoop` _activationobjects)
    (:`LoopBody`
      (`/Engine/EditorBlueprintResources/StandardMacros.IsValid` _array_element
        (:`Is Not Valid`
          (`KismetArrayLibrary.Array_Remove` _activationobjects _array_index))))
    (:`Completed`
      (bind (_array_element_2 _array_index_2) (`/Game/Gameplay/BPML_CustomMacros.ReverseForEachLoop` _activationpads)
        (:`LoopBody`
          (`/Engine/EditorBlueprintResources/StandardMacros.IsValid` _array_element_2
            (:`Is Not Valid`
              (`KismetArrayLibrary.Array_Remove` _activationpads _array_index_2))))))))

(event `self.ReceiveActorBeginOverlap`
  (params (OtherActor :type "Actor Object Reference")))

(event `self.LightOnFire`
  (`parent.LightOnFire`))

(event `self.ExtinguishFire`)

(event `self.ThisTorchIsOn`)

(event `self.ThisTorchIsOff`)

(event `self.AddOne`
  (`|ExecutionSequence`
    (:`then_0`
      (for _array_element (`self.ActivationObjects`)
        (`/Engine/EditorBlueprintResources/StandardMacros.IsValid` _array_element
          (:`Is Valid`
            (`/Game/Gameplay/BP_ActivatedByTorches.AddOneTorch` _array_element)))))
    (:`then_1`
      (for _array_element_2 (`self.ActivationPads`)
        (`/Engine/EditorBlueprintResources/StandardMacros.IsValid` _array_element_2
          (:`Is Valid`
            (`/Game/Gameplay/SpinPads/BP_SpinPadNeedsTorchActivation.Pad_AddOneTorch` _array_element_2)))))))

(event `self.SubtractOne`
  (`|ExecutionSequence`
    (:`then_0`
      (for _array_element (`self.ActivationObjects`)
        (`/Engine/EditorBlueprintResources/StandardMacros.IsValid` _array_element
          (:`Is Valid`
            (`/Game/Gameplay/BP_ActivatedByTorches.SubtractOneTorch` _array_element)))))
    (:`then_1`
      (for _array_element_2 (`self.ActivationPads`)
        (`/Engine/EditorBlueprintResources/StandardMacros.IsValid` _array_element_2
          (:`Is Valid`
            (`/Game/Gameplay/SpinPads/BP_SpinPadNeedsTorchActivation.Pad_SubtractOneTorch` _array_element_2)))))))

(fn `UserConstructionScript`
  (bind _activationobjects (`self.ActivationObjects`))
  (bind _activationpads (`self.ActivationPads`))
  (`parent.UserConstructionScript`)
  (`|ExecutionSequence`
    (:`then_0`
      (if (!= (`KismetArrayLibrary.Array_Length` _activationobjects) 0)
        (for _array_element _activationobjects
          (`/Engine/EditorBlueprintResources/StandardMacros.IsValid` _array_element
            (:`Is Valid`
              (`KismetArrayLibrary.Array_AddUnique` (`/Game/Gameplay/BP_ActivatedByTorches.DoNotEditThisArray_TorchesNeeded` _array_element) self)))))
      (bind _outactors (`GameplayStatics.GetAllActorsOfClass` "/Game/Gameplay/BP_ActivatedByTorches.BP_ActivatedByTorches_C"))
      (bind _array_element_2 (`/Game/Gameplay/BPML_CustomMacros.ReverseForEachLoop` _outactors)
        (:`LoopBody`
          (bind _donoteditthisarray_torchesneeded (`/Game/Gameplay/BP_ActivatedByTorches.DoNotEditThisArray_TorchesNeeded` _array_element_2))
          (if (and (`KismetArrayLibrary.Array_Contains` _donoteditthisarray_torchesneeded self) (not (`KismetArrayLibrary.Array_Contains` (`self.ActivationObjects`) _array_element_2)))
            (`KismetArrayLibrary.Array_RemoveItem` _donoteditthisarray_torchesneeded self)))
        (:`Completed`
          (for _array_element_3 (`self.ActivationObjects`)
            (set `/Game/Gameplay/BP_ActivatedByTorches.NumTorchesNeeded` (`KismetArrayLibrary.Array_Length` (`/Game/Gameplay/BP_ActivatedByTorches.DoNotEditThisArray_TorchesNeeded` _array_element_3)) _array_element_3)))))
    (:`then_1`
      (if (!= (`KismetArrayLibrary.Array_Length` _activationpads) 0)
        (for _array_element_4 _activationpads
          (`/Engine/EditorBlueprintResources/StandardMacros.IsValid` _array_element_4
            (:`Is Valid`
              (`KismetArrayLibrary.Array_AddUnique` (`/Game/Gameplay/SpinPads/BP_SpinPadNeedsTorchActivation.DoNotEditThisArray_TorchesNeeded` _array_element_4) self)))))
      (bind _outactors_2 (`GameplayStatics.GetAllActorsOfClass` "/Game/Gameplay/SpinPads/BP_SpinPadNeedsTorchActivation.BP_SpinPadNeedsTorchActivation_C"))
      (bind _array_element_5 (`/Game/Gameplay/BPML_CustomMacros.ReverseForEachLoop` _outactors_2)
        (:`LoopBody`
          (bind _donoteditthisarray_torchesneeded_2 (`/Game/Gameplay/SpinPads/BP_SpinPadNeedsTorchActivation.DoNotEditThisArray_TorchesNeeded` _array_element_5))
          (if (and (`KismetArrayLibrary.Array_Contains` _donoteditthisarray_torchesneeded_2 self) (not (`KismetArrayLibrary.Array_Contains` (`self.ActivationPads`) _array_element_5)))
            (`KismetArrayLibrary.Array_RemoveItem` _donoteditthisarray_torchesneeded_2 self)))
        (:`Completed`
          (for _array_element_6 (`self.ActivationPads`)
            (set `/Game/Gameplay/SpinPads/BP_SpinPadNeedsTorchActivation.NumTorchesNeeded` (`KismetArrayLibrary.Array_Length` (`/Game/Gameplay/SpinPads/BP_SpinPadNeedsTorchActivation.DoNotEditThisArray_TorchesNeeded` _array_element_6)) _array_element_6)))))))