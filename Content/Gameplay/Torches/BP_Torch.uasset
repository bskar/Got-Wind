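; Torch actor that can be lit or extinguished, toggling its fire effect and adjusting the lit-torch count on an optional TreeToBurn.
; When a lit torch overlaps a BP_TestWeapon that can spread fire, it consumes that flag and spawns a normal or upgraded fireball along the player's facing.
; The construction script draws persistent debug circles estimating both fireballs' reach from hardcoded speed, lifetime and collision radii, aiding torch placement.
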(event `LightOnFire`
  (bind _torchfireeffect (`self.TorchFireEffect`))
  (if (not (`self.IsLit`))
    (`ParticleSystemComponent.SetTemplate` _torchfireeffect "/Game/InfinityBladeEffects/Effects/FX_Combat_Base/WeaponShimmer/Fire/P_WeaponShimmer_Fire_Blunt.P_WeaponShimmer_Fire_Blunt")
    (`ActorComponent.Activate` _torchfireeffect false)
    (set `self.IsLit` true)
    (`/Engine/EditorBlueprintResources/StandardMacros.IsValid` (`self.TreeToBurn`)
      (:`Is Valid`
        (`/Game/Gameplay/BP_BurningTree.AddOneTorch` (`self.TreeToBurn`))))))

(event `self.ReceiveBeginPlay`
  (bind _torchfireeffect (`self.TorchFireEffect`))
  (if (not (`self.IsLit`))
    (`ActorComponent.Deactivate` _torchfireeffect)
    (`ParticleSystemComponent.SetTemplate` _torchfireeffect null)))

(event `self.ReceiveActorBeginOverlap`
  (params (OtherActor :type "Actor Object Reference"))
  (bind _returnvalue (`KismetMathLibrary.MakeTransform` (`SceneComponent.K2_GetComponentLocation` (`self.TorchFireEffect`)) (`self.K2_GetActorRotation` (`GameplayStatics.GetPlayerCharacter` 0))))
  (if (`self.IsLit`)
    (bind _asbp_test_weapon (cast `/Game/Weapons/BP_TestWeapon` OtherActor))
    (if (`/Game/Weapons/BP_TestWeapon.CanSpreadFire` _asbp_test_weapon)
      (set `/Game/Weapons/BP_TestWeapon.CanSpreadFire` false _asbp_test_weapon)
      (if (`/Game/Weapons/BP_TestWeapon.HasFireballUpgrade` _asbp_test_weapon)
        (`|SpawnActorFromClass` "/Game/Gameplay/Fireballs/BP_TorchFireballPlus.BP_TorchFireballPlus_C" _returnvalue "Undefined" "OverrideRootScale")
        (else
          (`|SpawnActorFromClass` "/Game/Gameplay/Fireballs/BP_TorchFireball.BP_TorchFireball_C" _returnvalue "Undefined" "OverrideRootScale"))))))

(event `ExtinguishFire`
  (bind _torchfireeffect (`self.TorchFireEffect`))
  (if (`self.IsLit`)
    (`ActorComponent.Deactivate` _torchfireeffect)
    (`ParticleSystemComponent.SetTemplate` _torchfireeffect null)
    (set `self.IsLit` false)
    (`/Engine/EditorBlueprintResources/StandardMacros.IsValid` (`self.TreeToBurn`)
      (:`Is Valid`
        (`/Game/Gameplay/BP_BurningTree.SubtractOneTorch` (`self.TreeToBurn`))))))

(fn `UserConstructionScript`
  (bind _sphereradius (`SphereComponent.SphereRadius` (`self.TorchFireTrigger`)))
  (`KismetSystemLibrary.FlushPersistentDebugLines`)
  (`KismetSystemLibrary.DrawDebugCircle` (`SceneComponent.K2_GetComponentLocation` (`self.TorchFireTrigger`)) (+ (* 540.0 1.0) 21.0 _sphereradius) 64 (struct :`R` 1.0 :`G` 0.5 :`A` 1.0) 61440.0 2.8 (0.0 1.0 0.0) (1.0 0.0 0.0))
  (`KismetSystemLibrary.DrawDebugCircle` (`SceneComponent.K2_GetComponentLocation` (`self.TorchFireTrigger`)) (+ (* 540.0 2.0) 30.0 _sphereradius) 128 (struct :`R` 1.0 :`A` 1.0) 61440.0 2.8 (0.0 1.0 0.0) (1.0 0.0 0.0) true))