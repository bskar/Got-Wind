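; BP_TorchLongRange is a child torch Blueprint, named as a long-range variant of a torch that can be lit and extinguished.
; Its begin play, overlap, fire and on/off state events, along with its construction script, only forward to the parent.
; It adds no graph logic of its own, so all visible behavior is inherited from the parent torch.
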(event `self.ReceiveBeginPlay`
  (`parent.ReceiveBeginPlay`))

(event `self.ReceiveActorBeginOverlap`
  (params (OtherActor :type "Actor Object Reference"))
  (`parent.ReceiveActorBeginOverlap` OtherActor))

(event `self.LightOnFire`
  (`parent.LightOnFire`))

(event `self.ExtinguishFire`
  (`parent.ExtinguishFire`))

(event `self.ThisTorchIsOn`
  (`parent.ThisTorchIsOn`))

(event `self.ThisTorchIsOff`
  (`parent.ThisTorchIsOff`))

(fn `UserConstructionScript`
  (`parent.UserConstructionScript`))