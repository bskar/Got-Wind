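; Windstone particle actor that homes in on the player character's Fan component after spawning.
; A timeline, rate-scaled by SecondsToReachFullSpeed, ramps the VInterpTo speed so the pull starts slow and accelerates while tracking the Fan's current location.
; Overlapping a ThirdPersonCharacter deactivates its three particle systems, then destroys the actor after a short delay to let the effects fade.
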(event `self.ReceiveBeginPlay`
  (`TimelineComponent.SetPlayRate` (`self.HomingGraph`) (/ 1.0 (`self.SecondsToReachFullSpeed`)))
  (bind (_direction _homingtrack) (`Timeline|HomingGraph` :!via `PlayFromStart`)
    (:`Update`
      (`self.K2_SetActorLocation` (`KismetMathLibrary.VInterpTo` (`self.K2_GetActorLocation`) (`SceneComponent.K2_GetComponentLocation` (`/Game/Characters/Player/ThirdPersonCharacter.Fan` (cast `/Game/Characters/Player/ThirdPersonCharacter` (`GameplayStatics.GetPlayerCharacter` 0) :!pure true))) (`GameplayStatics.GetWorldDeltaSeconds`) (`KismetMathLibrary.Lerp` 0.1 14.0 _homingtrack))))
    (:`Finished`)))

(event `self.ReceiveActorBeginOverlap`
  (params (OtherActor :type "Actor Object Reference"))
  (cast `/Game/Characters/Player/ThirdPersonCharacter` OtherActor)
  (`ActorComponent.Deactivate` (`self.ParticleSystem`))
  (`ActorComponent.Deactivate` (`self.ParticleSystem1`))
  (`ActorComponent.Deactivate` (`self.ParticleSystem2`))
  (`KismetSystemLibrary.Delay` 2.4)
  (`self.K2_DestroyActor`))

(fn `UserConstructionScript`)