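; Spin pad variant, apparently tied to torches, that can light a set of torches with a brief effect.
; LightPadTorches activates the spin effect, lights every entry in TorchesToLight, then switches the effect off after a short delay.
; A DoOnce blocks retriggering until that delay ends.
; Torch add and subtract events only call the parent, and the Activate override leads to an empty DoOnce.
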(event `self.AddOneTorch`
  (`parent.AddOneTorch`))

(event `self.SubtractOneTorch`
  (`parent.SubtractOneTorch`))

(event `self.Activate`
  (`/Engine/EditorBlueprintResources/StandardMacros.DoOnce` false))

(event `LightPadTorches`
  (`/Engine/EditorBlueprintResources/StandardMacros.DoOnce` false :!label _label
    (:`Completed`
      (`ActorComponent.Activate` (`self.SpinPadEffect`) false)
      (for _array_element (`self.TorchesToLight`)
        (`/Game/Gameplay/Torches/BP_TorchBase.LightOnFire` _array_element))
      (`KismetSystemLibrary.Delay` 1.2)
      (`ActorComponent.Deactivate` (`self.SpinPadEffect`))
      (goto _label :!via `Reset`))))

(fn `UserConstructionScript`
  (`parent.UserConstructionScript`))