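; Base projectile actor that lights torches and kills imps it overlaps.
; It arms after a creation delay, then expires via Impact when its lifetime ends or it hits either target, disabling collision response, deactivating its effect and destroying itself after a death delay.
; The construction script scales lifetime by a range multiplier, compensating for creation time; nodes that would scale movement speed are unconnected.
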(event `self.ReceiveBeginPlay`
  (`KismetSystemLibrary.Delay` (`self.Creationtime`))
  (set `self.CanImpact` true)
  (`KismetSystemLibrary.Delay` (`self.Lifetime`))
  (`self.Impact`))

(event `Impact`
  (`ActorComponent.Deactivate` (`self.ProjectileEffect`))
  (set `self.CanImpact` false)
  (`KismetSystemLibrary.Delay` (`self.Deathtime`))
  (`self.K2_DestroyActor`))

(event `self.ReceiveActorBeginOverlap`
  (params (OtherActor :type "Actor Object Reference"))
  (if (`self.CanImpact`)
    (bind _asbp_torch_base (cast `/Game/Gameplay/Torches/BP_TorchBase` OtherActor)
      (:`then`
        (`/Game/Gameplay/Torches/BP_TorchBase.LightOnFire` _asbp_torch_base)
        (`self.Impact`))
      (:`CastFailed`
        (bind _asbp_imp (cast `/Game/Characters/NPC/Imp/BP_Imp` OtherActor))
        (`/Game/Characters/NPC/Imp/BP_Imp.Die` _asbp_imp)
        (`self.Impact`)))))

(fn `UserConstructionScript`
  (set `self.Lifetime` (+ (* (`self.Lifetime`) (`self.RangeMultiplier`)) (* (`self.Creationtime`) (- (`self.RangeMultiplier`) 1.0)))))