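; BP_Windstone is a windstone actor that releases its power to the player character, BP_Vayu.
; ReleasePower sets Vayu's Progress to a configured value, spawns a configurable number of particle actors at random nearby offsets flagged to go to Vayu, then fires a radial force impulse.
; The construction script applies configurable outside and inside materials to the stone mesh.
; Nothing in this graph triggers the release; a delayed call is left disconnected.
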(event `self.ReceiveBeginPlay`)

(event `ReleasePower`
  (bind _returnvalue (`KismetMathLibrary.RandomFloatInRange` 0.0 100.0))
  (set `/Game/Characters/Player/BP_Vayu.Progress` (`self.ProgressToSet`) (cast `/Game/Characters/Player/BP_Vayu` (`GameplayStatics.GetPlayerCharacter` 0) :!pure true))
  (for _ (range 1 (+ (`self.NumPowerParticles`) 1))
    (`|SpawnActorFromClass` "/Game/Gameplay/BP_WindstoneParticles.BP_WindstoneParticles_C" (`KismetMathLibrary.MakeTransform` (`KismetMathLibrary.MakeVector` (+ _returnvalue (.x (`self.K2_GetActorLocation`))) (+ _returnvalue (.y (`self.K2_GetActorLocation`))) (+ (.z (`self.K2_GetActorLocation`)) (`KismetMathLibrary.RandomFloatInRange` 0.0 75.0)))) "Undefined" "OverrideRootScale" null true))
  (`RadialForceComponent.FireImpulse` (`self.RadialForce`)))

(fn `UserConstructionScript`
  (`PrimitiveComponent.SetMaterial` (`self.SM_WindStone_01_DM`) 0 (`self.OutsideMaterial`))
  (`PrimitiveComponent.SetMaterial` (`self.SM_WindStone_01_DM`) 1 (`self.InsideMaterial`)))