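; Wheel that the player's wind slashes turn to raise or lower a linked Chimes actor until it is fully open.
; Each BP_WindSlash counts once and restarts a timeline that spins the wheel and offsets the Chimes in Lerp-scaled per-update steps.
; A clamped position counter stops motion permanently at OpenDistance; only Up and Down gate types move.
; The construction script draws a debug line linking wheel and Chimes.
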(event `self.ReceiveBeginPlay`
  (set `self.OpenDistance` (`KismetMathLibrary.Abs` (`self.OpenDistance`)))
  (bind _output_get (set `self.CurrentPosition` (.z (`self.K2_GetActorLocation` (`self.Chimes`)))))
  (bind _output_get_2 (set `self.ClosedPosition` _output_get))
  (set `self.OpenPosition` (+ _output_get_2 (`self.OpenDistance`))))

(event `self.ReceiveActorBeginOverlap`
  (params (OtherActor :type "Actor Object Reference"))
  (bind _chimes (`self.Chimes`))
  (bind _asbp_wind_slash (cast `/Game/Weapons/BP_WindSlash` OtherActor))
  (if (`/Game/Weapons/BP_WindSlash.CanTurnWheel` _asbp_wind_slash)
    (set `/Game/Weapons/BP_WindSlash.CanTurnWheel` false _asbp_wind_slash)
    (if (`self.IsFullyOpened`)
      _
      (elif (`self.IsTurning`)
        (bind (_direction _opentrack) (`Timeline|OpenGraph` :!via `PlayFromStart` :!label _label)
          (:`Update`
            (bind _returnvalue (`KismetMathLibrary.Lerp` 6.5 0.5 _opentrack))
            (bind _output_get (set `self.CurrentPosition` (`KismetMathLibrary.FClamp` (+ (`self.CurrentPosition`) _returnvalue) (`self.ClosedPosition`) (`self.OpenPosition`))))
            (if (< _output_get (`self.OpenPosition`))
              (`SceneComponent.K2_AddLocalRotation` (`self.WheelCenter`) (`KismetMathLibrary.MakeRotator` 0.0 0.0 _returnvalue) false false)
              (switch `/Game/Gameplay/E_GateType` (`self.GateType`)
                (:`NewEnumerator0`
                  (`self.K2_AddActorLocalOffset` _chimes (`KismetMathLibrary.MakeVector` 0.0 0.0 _returnvalue) false false))
                (:`NewEnumerator1`
                  (`self.K2_AddActorLocalOffset` _chimes (`KismetMathLibrary.MakeVector` 0.0 0.0 (* _returnvalue -1.0)) false false)))
              (else
                (`self.StopOpening`)
                (set `self.IsFullyOpened` true)
                (set `self.IsTurning` false))))
          (:`Finished`
            (set `self.IsTurning` false)))
        (else
          (set `self.IsTurning` true)
          (goto _label :!via `PlayFromStart`))))))

(event `StopOpening`
  (goto _label :!via `Stop`))

(event `self.WheelTriggerUp.OnComponentBeginOverlap`
  (params (OtherActor :type "Actor Object Reference") (OtherComp :type "PrimitiveComponent Object Reference") (OtherBodyIndex :type Integer) (bFromSweep :type Boolean) (SweepResult :type "HitResult Structure (by ref)")))

(event `self.WheelTriggerUp.OnComponentHit`
  (params (OtherActor :type "Actor Object Reference") (OtherComp :type "PrimitiveComponent Object Reference") (NormalImpulse :type "Vector Structure") (Hit :type "HitResult Structure (by ref)")))

(event `self.WheelTriggerDown.OnComponentBeginOverlap`
  (params (OtherActor :type "Actor Object Reference") (OtherComp :type "PrimitiveComponent Object Reference") (OtherBodyIndex :type Integer) (bFromSweep :type Boolean) (SweepResult :type "HitResult Structure (by ref)")))

(event `self.WheelTriggerDown.OnComponentHit`
  (params (OtherActor :type "Actor Object Reference") (OtherComp :type "PrimitiveComponent Object Reference") (NormalImpulse :type "Vector Structure") (Hit :type "HitResult Structure (by ref)")))

(fn `UserConstructionScript`
  (bind _chimes (`self.Chimes`))
  (set `self.OpenDistance` (`KismetMathLibrary.Abs` (`self.OpenDistance`)))
  (bind _output_get (set `self.CurrentPosition` (.z (`self.K2_GetActorLocation` (`self.Chimes`)))))
  (bind _output_get_2 (set `self.ClosedPosition` _output_get))
  (set `self.OpenPosition` (+ _output_get_2 (`self.OpenDistance`)))
  (`KismetSystemLibrary.FlushPersistentDebugLines`)
  (`/Engine/EditorBlueprintResources/StandardMacros.IsValid` _chimes
    (:`Is Valid`
      (`KismetSystemLibrary.DrawDebugLine` (+ (`self.K2_GetActorLocation`) (0.0 0.0 100.0)) (`self.K2_GetActorLocation` _chimes) (struct :`G` 1.0 :`B` 0.000452 :`A` 1.0) 61440.0 4.2))))