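; BP_Checkpoint is a numbered checkpoint actor that sets a ThirdPersonCharacter's CheckpointNum to its own Number on overlap, with no check on the previous value.
; Its construction script clamps negative numbers to zero and prints a warning when another checkpoint shares the same non-zero number.
; It also writes the prefixed number to NumberText and adjusts one text axis by the root's Y/Z scale ratio to offset non-uniform scaling.
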(event `self.ReceiveActorBeginOverlap`
  (params (OtherActor :type "Actor Object Reference"))
  (bind _asthird_person_character (cast `/Game/Dev/ThirdPersonBP/Blueprints/ThirdPersonCharacter` OtherActor))
  (set `/Game/Dev/ThirdPersonBP/Blueprints/ThirdPersonCharacter.CheckpointNum` (`self.Number`) _asthird_person_character))

(fn `UserConstructionScript`
  (bind _numbertext (`self.NumberText`))
  (bind _y (.y (`SceneComponent.K2_GetComponentScale` (`self.DefaultSceneRoot`))))
  (bind _z (.z (`SceneComponent.K2_GetComponentScale` (`self.DefaultSceneRoot`))))
  (if (< (`self.Number`) 0)
    (set `self.Number` 0))
  (if (!= (`self.Number`) 0)
    (bind _outactors (`GameplayStatics.GetAllActorsOfClass` "BP_Checkpoint_C"))
    (for _array_element _outactors
      (if (and (== (`/Game/Gameplay/BP_Checkpoint.Number` _array_element) (`self.Number`)) (!= _array_element self))
        (`KismetSystemLibrary.PrintString` (`KismetStringLibrary.Concat_StrStr` "Warning: This Checkpoint number ( #" (`KismetStringLibrary.Conv_IntToString` (`self.Number`)) " ) already exists!") true true (struct :`G` 0.66 :`B` 1.0 :`A` 1.0) 8.4))))
  (`TextRenderComponent.K2_SetText` _numbertext (`KismetTextLibrary.Conv_StringToText` (`KismetStringLibrary.Concat_StrStr` (`self.Prefix`) (`KismetStringLibrary.Conv_IntToString` (`self.Number`)))))
  (if (>= _y _z)
    (`TextRenderComponent.SetYScale` _numbertext (/ _y _z))
    (else
      (`TextRenderComponent.SetXScale` _numbertext (/ _z _y)))))