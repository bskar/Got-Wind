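; Spin pad variant that opens a linked Gate once when activated, briefly running its effect as the gate opens.
; ActivatePad fires through a DoOnce and calls Open on a closed gate; Close is an empty stub, with its old logic disconnected.
; A timeline pulses the symbol material's emissive or MaxGlow pins it bright, until activation resets the glow and shuts both flow gates against further changes.
; Overlap events defer to the parent class.
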(event `self.ReceiveActorBeginOverlap`
  (params (OtherActor :type "Actor Object Reference"))
  (`parent.ReceiveActorBeginOverlap` OtherActor))

(event `self.ReceiveActorEndOverlap`
  (params (OtherActor :type "Actor Object Reference"))
  (`parent.ReceiveActorEndOverlap` OtherActor))

(event `self.ActivatePad`
  (`/Engine/EditorBlueprintResources/StandardMacros.DoOnce` false
    (:`Completed`
      (`ActorComponent.Activate` (`self.SpinPadEffect`) false)
      (if (`self.IsClosed`)
        (`self.Open`)
        (else
          (`self.Close`)))
      (`self.NoGlow`))))

(event `Open`
  (if (`self.IsClosed`)
    (set `self.IsClosed` false)
    (`/Game/Gameplay/BP_SymbolGate.OpenSesame` (`self.Gate`))
    (`KismetSystemLibrary.Delay` 1.2)
    (`ActorComponent.Deactivate` (`self.SpinPadEffect`))))

(event `Close`)

(event `self.StartPulsing`
  (`/Engine/EditorBlueprintResources/StandardMacros.Gate` false :!label _label
    (:`Exit`
      (bind (_direction _pulsetrack) (`Timeline|PulseGraph` :!via `PlayFromStart` :!label _label_2)
        (:`Update`
          (`MaterialInstanceDynamic.SetScalarParameterValue` (`self.SymbolMaterial`) "Emissive_Strength" (`KismetMathLibrary.Lerp` 6.0 100.0 _pulsetrack)))))))

(event `self.MaxGlow`
  (`/Engine/EditorBlueprintResources/StandardMacros.Gate` false :!label _label_3
    (:`Exit`
      (`|ExecutionSequence`
        (:`then_0`
          (goto _label_2 :!via `Stop`))
        (:`then_1`
          (`MaterialInstanceDynamic.SetScalarParameterValue` (`self.SymbolMaterial`) "Emissive_Strength" 142.0))))))

(event `self.NoGlow`
  (`|ExecutionSequence`
    (:`then_0`
      (goto _label :!via `Close`))
    (:`then_1`
      (goto _label_3 :!via `Close`))
    (:`then_2`
      (goto _label_2 :!via `Stop`))
    (:`then_3`
      (`MaterialInstanceDynamic.SetScalarParameterValue` (`self.SymbolMaterial`) "Emissive_Strength" 6.0))))

(fn `UserConstructionScript`
  (`parent.UserConstructionScript`))