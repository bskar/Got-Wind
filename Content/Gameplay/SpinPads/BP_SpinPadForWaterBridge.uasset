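; BP_SpinPadForWaterBridge is a spin pad that rotates a referenced Bridge actor when activated.
; Activation or Skipped fires once, playing the pad effect, calling Down or Up by IsUp state, then clearing the glow.
; Down eases bridge roll to a fixed angle via timeline, while Up is empty.
; Gated events drive symbol emissive pulsing and max glow until NoGlow closes both gates.
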(event `self.ReceiveActorBeginOverlap`
  (params (OtherActor :type "Actor Object Reference"))
  (`parent.ReceiveActorBeginOverlap` OtherActor))

(event `self.ReceiveActorEndOverlap`
  (params (OtherActor :type "Actor Object Reference"))
  (`parent.ReceiveActorEndOverlap` OtherActor))

(event `self.ActivatePad`
  (`/Engine/EditorBlueprintResources/StandardMacros.DoOnce` false :!label _label
    (:`Completed`
      (`ActorComponent.Activate` (`self.SpinPadEffect`) false)
      (if (`self.IsUp`)
        (`self.Down`)
        (else
          (`self.Up`)))
      (`self.NoGlow`))))

(event `Skipped`
  (goto _label))

(event `Down`
  (if (`self.IsUp`)
    (set `self.IsUp` false)
    (set `self.DefaultRotation` (.roll (`self.K2_GetActorRotation` (`self.Bridge`))))
    (`|ExecutionSequence`
      (:`then_0`
        (`KismetSystemLibrary.Delay` 1.2)
        (`ActorComponent.Deactivate` (`self.SpinPadEffect`)))
      (:`then_1`
        (bind (_direction _bridgerotatetrack) (`Timeline|BridgeRotateGraph` :!via `PlayFromStart`)
          (:`Update`
            (`self.SetActorRotation` (`self.Bridge`) (`KismetMathLibrary.MakeRotator` (`KismetMathLibrary.Lerp` (`self.DefaultRotation`) -90.0 _bridgerotatetrack) (.pitch (`self.K2_GetActorRotation` (`self.Bridge`))) (.yaw (`self.K2_GetActorRotation` (`self.Bridge`)))))))))))

(event `Up`)

(event `self.StartPulsing`
  (`/Engine/EditorBlueprintResources/StandardMacros.Gate` false :!label _label_2
    (:`Exit`
      (bind (_direction _pulsetrack) (`Timeline|PulseGraph` :!via `PlayFromStart` :!label _label_3)
        (:`Update`
          (`MaterialInstanceDynamic.SetScalarParameterValue` (`self.SymbolMaterial`) "Emissive_Strength" (`KismetMathLibrary.Lerp` 6.0 100.0 _pulsetrack)))))))

(event `self.MaxGlow`
  (`/Engine/EditorBlueprintResources/StandardMacros.Gate` false :!label _label_4
    (:`Exit`
      (`|ExecutionSequence`
        (:`then_0`
          (goto _label_3 :!via `Stop`))
        (:`then_1`
          (`MaterialInstanceDynamic.SetScalarParameterValue` (`self.SymbolMaterial`) "Emissive_Strength" 142.0))))))

(event `self.NoGlow`
  (`|ExecutionSequence`
    (:`then_0`
      (goto _label_2 :!via `Close`))
    (:`then_1`
      (goto _label_4 :!via `Close`))
    (:`then_2`
      (goto _label_3 :!via `Stop`))
    (:`then_3`
      (`MaterialInstanceDynamic.SetScalarParameterValue` (`self.SymbolMaterial`) "Emissive_Strength" 6.0))))

(fn `UserConstructionScript`
  (`parent.UserConstructionScript`))