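; Spin pad child Blueprint that, when activated, makes its linked dragons fire together.
; ActivatePad fires only if every dragon in DragonsToActivate is ready, playing the pad effect briefly; otherwise it prints a failure message.
; A DoOnce blocks re-entry until each attempt finishes.
; Glow events drive the symbol material's emissive through a pulsing timeline, maximum or dim; NoGlow also closes the gate that admits pulsing.
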(event `self.ReceiveActorBeginOverlap`
  (params (OtherActor :type "Actor Object Reference"))
  (`parent.ReceiveActorBeginOverlap` OtherActor))

(event `self.ReceiveActorEndOverlap`
  (params (OtherActor :type "Actor Object Reference"))
  (`parent.ReceiveActorEndOverlap` OtherActor))

(event `self.ActivatePad`
  (`/Engine/EditorBlueprintResources/StandardMacros.DoOnce` false :!label _label
    (:`Completed`
      (set `self.CanFire` true)
      (for _array_element (`self.DragonsToActivate`)
        (if (not (`/Game/Gameplay/Torches/BP_TorchDragonSpecial.IsReadyToFire` _array_element))
          (set `self.CanFire` false)))
      (if (`self.CanFire`)
        (`ActorComponent.Activate` (`self.SpinPadEffect`) false)
        (for _array_element_2 (`self.DragonsToActivate`)
          (`/Game/Gameplay/Torches/BP_TorchBase.DragonFire` _array_element_2))
        (`KismetSystemLibrary.Delay` 1.2)
        (`ActorComponent.Deactivate` (`self.SpinPadEffect`))
        (goto _label :!via `Reset`)
        (else
          (`KismetSystemLibrary.PrintString` "I can't do it, Captain!")
          (goto _label :!via `Reset`))))))

(event `self.StartPulsing`
  (`/Engine/EditorBlueprintResources/StandardMacros.Gate` false :!label _label_2
    (:`Exit`
      (bind (_direction _pulsetrack) (`Timeline|PulseGraph` :!via `PlayFromStart` :!label _label_3)
        (:`Update`
          (`MaterialInstanceDynamic.SetScalarParameterValue` (`self.SymbolMaterial`) "Emissive_Strength" (`KismetMathLibrary.Lerp` 16.0 100.0 _pulsetrack)))))))

(event `self.MaxGlow`
  (`|ExecutionSequence`
    (:`then_0`
      (goto _label_3 :!via `Stop`))
    (:`then_1`
      (`MaterialInstanceDynamic.SetScalarParameterValue` (`self.SymbolMaterial`) "Emissive_Strength" 210.0))))

(event `self.NoGlow`
  (`|ExecutionSequence`
    (:`then_0`
      (goto _label_2 :!via `Close`))
    (:`then_1`
      (goto _label_3 :!via `Stop`))
    (:`then_2`
      (`MaterialInstanceDynamic.SetScalarParameterValue` (`self.SymbolMaterial`) "Emissive_Strength" 16.0))))

(fn `UserConstructionScript`
  (`parent.UserConstructionScript`))