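; BP_SpinPadForTorch is a spin pad variant that lights a set of linked torches when activated.
; ActivatePad plays the SpinPadEffect, calls LightOnFire on each entry in TorchesToLight, then switches the effect off after a short delay.
; A DoOnce gate blocks retriggering until that delay ends, while overlap handling is left to the parent class.
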(event `self.ReceiveActorBeginOverlap`
  (params (OtherActor :type "Actor Object Reference"))
  (`parent.ReceiveActorBeginOverlap` OtherActor))

(event `self.ReceiveActorEndOverlap`
  (params (OtherActor :type "Actor Object Reference"))
  (`parent.ReceiveActorEndOverlap` OtherActor))

(event `self.ActivatePad`
  (`/Engine/EditorBlueprintResources/StandardMacros.DoOnce` false :!label _label
    (:`Completed`
      (`ActorComponent.Activate` (`self.SpinPadEffect`) false)
      (for _array_element (`self.TorchesToLight`)
        (`/Game/Gameplay/Torches/BP_TorchBase.LightOnFire` _array_element))
      (`KismetSystemLibrary.Delay` 1.2)
      (`ActorComponent.Deactivate` (`self.SpinPadEffect`))
      (goto _label :!via `Reset`))))

(fn `UserConstructionScript`
  (`parent.UserConstructionScript`))