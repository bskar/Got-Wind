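; A child spin pad that stays locked until all its linked torches are burning, then can be activated to light other torches with a brief effect.
; Torch add and subtract events track the lit count; reaching the required total unlocks activation and pulses the symbol's emissive glow through a gated timeline.
; The construction script prunes invalid torch references and draws debug lines to each required torch.
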(event `self.ReceiveBeginPlay`
  (bind _donoteditthisarray_torchesneeded (`self.DoNotEditThisArray_TorchesNeeded`))
  (bind (_array_element _array_index) (`/Game/Gameplay/BPML_CustomMacros.ReverseForEachLoop` _donoteditthisarray_torchesneeded)
    (:`LoopBody`
      (`/Engine/EditorBlueprintResources/StandardMacros.IsValid` _array_element
        (:`Is Not Valid`
          (`KismetArrayLibrary.Array_Remove` _donoteditthisarray_torchesneeded _array_index))))
    (:`Completed`
      (set `self.NumTorchesNeeded` (`KismetArrayLibrary.Array_Length` (`self.DoNotEditThisArray_TorchesNeeded`))))))

(event `self.ReceiveActorBeginOverlap`
  (params (OtherActor :type "Actor Object Reference"))
  (`parent.ReceiveActorBeginOverlap` OtherActor))

(event `self.ReceiveActorEndOverlap`
  (params (OtherActor :type "Actor Object Reference"))
  (`parent.ReceiveActorEndOverlap` OtherActor))

(event `self.ActivatePad`
  (`/Engine/EditorBlueprintResources/StandardMacros.DoOnce` true :!label _label
    (:`Completed`
      (`ActorComponent.Activate` (`self.SpinPadEffect`) false)
      (for _array_element (`self.TorchesToLight`)
        (`/Game/Gameplay/Torches/BP_TorchBase.LightOnFire` _array_element))
      (`KismetSystemLibrary.Delay` 1.2)
      (`ActorComponent.Deactivate` (`self.SpinPadEffect`))
      (goto _label :!via `Reset`))))

(event `Pad_AddOneTorch`
  (bind _result (`/Engine/EditorBlueprintResources/StandardMacros.IncrementInt` (`self.NumTorchesOnFire`))
    (:`  `
      (`/Engine/EditorBlueprintResources/StandardMacros.CompareInt` _result (`self.NumTorchesNeeded`)
        (:`==`
          (`self.TorchActivatePad`))))))

(event `Pad_SubtractOneTorch`
  (`/Engine/EditorBlueprintResources/StandardMacros.DecrementInt` (`self.NumTorchesOnFire`)))

(event `TorchActivatePad`
  (`/Engine/EditorBlueprintResources/StandardMacros.DoOnce` false
    (:`Completed`
      (`|ExecutionSequence`
        (:`then_0`
          (goto _label :!via `Reset`))
        (:`then_1`
          (goto _label_2 :!via `Open`))
        (:`then_2`
          (`self.StartPulsing`))))))

(event `self.StartPulsing`
  (`/Engine/EditorBlueprintResources/StandardMacros.Gate` true :!label _label_2
    (:`Exit`
      (bind (_direction _pulsetrack) (`Timeline|PulseGraph` :!via `PlayFromStart` :!label _label_3)
        (:`Update`
          (`MaterialInstanceDynamic.SetScalarParameterValue` (`self.SymbolMaterial`) "Emissive_Strength" (`KismetMathLibrary.Lerp` 12.0 100.0 _pulsetrack)))))))

(event `self.MaxGlow`
  (`|ExecutionSequence`
    (:`then_0`
      (goto _label_3 :!via `Stop`))
    (:`then_1`
      (`MaterialInstanceDynamic.SetScalarParameterValue` (`self.SymbolMaterial`) "Emissive_Strength" 155.0))))

(event `self.NoGlow`)

(fn `UserConstructionScript`
  (bind _donoteditthisarray_torchesneeded (`self.DoNotEditThisArray_TorchesNeeded`))
  (`parent.UserConstructionScript`)
  (bind (_array_element _array_index) (`/Game/Gameplay/BPML_CustomMacros.ReverseForEachLoop` _donoteditthisarray_torchesneeded)
    (:`LoopBody`
      (`/Engine/EditorBlueprintResources/StandardMacros.IsValid` _array_element
        (:`Is Not Valid`
          (`KismetArrayLibrary.Array_Remove` _donoteditthisarray_torchesneeded _array_index))))
    (:`Completed`
      (`KismetSystemLibrary.FlushPersistentDebugLines`)
      (for _array_element_2 (`self.DoNotEditThisArray_TorchesNeeded`)
        (`KismetSystemLibrary.DrawDebugLine` (`self.K2_GetActorLocation`) (+ (`self.K2_GetActorLocation` _array_element_2) (0.0 0.0 64.0)) (struct :`G` 1.0 :`B` 1.0 :`A` 1.0) 61440.0 2.8))
      (set `self.NumTorchesNeeded` (`KismetArrayLibrary.Array_Length` (`self.DoNotEditThisArray_TorchesNeeded`))))))