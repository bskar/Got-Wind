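; BP_SpinPadBase is a spin pad base class that registers itself with BP_Vayu while that actor overlaps it.
; Overlap begin sets Vayu's PadToActivate to this pad and enables CanActivate, and overlap end clears both.
; ActivatePad is an empty event, and the construction script applies GlowingMaterial to the SpinPadSymbol.
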(event `self.ReceiveActorBeginOverlap`
  (params (OtherActor :type "Actor Object Reference"))
  (bind _asbp_vayu (cast `/Game/Characters/Player/BP_Vayu` OtherActor))
  (set `/Game/Characters/Player/BP_Vayu.PadToActivate` self _asbp_vayu)
  (set `self.CanActivate` true))

(event `self.ReceiveActorEndOverlap`
  (params (OtherActor :type "Actor Object Reference"))
  (bind _asbp_vayu (cast `/Game/Characters/Player/BP_Vayu` OtherActor))
  (set `/Game/Characters/Player/BP_Vayu.PadToActivate` null _asbp_vayu)
  (set `self.CanActivate` false))

(event `ActivatePad`)

(fn `UserConstructionScript`
  (`PrimitiveComponent.SetMaterial` (`self.SpinPadSymbol`) 0 (`self.GlowingMaterial`)))