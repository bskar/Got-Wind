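; BP_TorchFireball is a projectile that ignites BP_Torch actors it overlaps.
; On BeginPlay it waits 1.0 minus Lifetime, enables CanLight, then expires after a further Lifetime delay.
; While CanLight is set, overlapping a torch calls LightOnFire.
; Both a hit and expiry deactivate FireballEffect, clear CanLight and destroy the actor after Deathtime.
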(event `self.ReceiveBeginPlay`
  (`KismetSystemLibrary.Delay` (- 1.0 (`self.Lifetime`)))
  (set `self.CanLight` true)
  (`KismetSystemLibrary.Delay` (`self.Lifetime`))
  (`ActorComponent.Deactivate` (`self.FireballEffect`))
  (set `self.CanLight` false)
  (`KismetSystemLibrary.Delay` (`self.Deathtime`))
  (`self.K2_DestroyActor`))

(event `self.ReceiveActorBeginOverlap`
  (params (OtherActor :type "Actor Object Reference"))
  (if (`self.CanLight`)
    (bind _asbp_torch (cast `/Game/Gameplay/BP_Torch` OtherActor))
    (`/Game/Gameplay/BP_Torch.LightOnFire` _asbp_torch)
    (`ActorComponent.Deactivate` (`self.FireballEffect`))
    (set `self.CanLight` false)
    (`KismetSystemLibrary.Delay` (`self.Deathtime`))
    (`self.K2_DestroyActor`)))

(fn `UserConstructionScript`)