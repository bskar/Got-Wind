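; Desert tower top hatch that appears and grows into a solid cover when the player character overlaps its trigger.
; The construction script disables the hatch's collision, then the first valid overlap unhides it and enables query and physics collision.
; A timeline then lerps its horizontal scale from tiny to full size while keeping it thin.
; A DoOnce makes the reveal one-shot, and a gate closes when the timeline finishes.
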(event `self.HatchTrigger.OnComponentBeginOverlap`
  (params (OtherActor :type "Actor Object Reference") (OtherComp :type "PrimitiveComponent Object Reference") (OtherBodyIndex :type Integer) (bFromSweep :type Boolean) (SweepResult :type "HitResult Structure (by ref)"))
  (bind _hatch (`self.Hatch`))
  (`/Engine/EditorBlueprintResources/StandardMacros.Gate` false :!label _label
    (:`Exit`
      (cast `/Game/Characters/Player/ThirdPersonCharacter` OtherActor)
      (`/Engine/EditorBlueprintResources/StandardMacros.DoOnce` false
        (:`Completed`
          (`SceneComponent.SetHiddenInGame` _hatch false true)
          (`SceneComponent.SetVisibility` _hatch true true)
          (`PrimitiveComponent.SetCollisionEnabled` _hatch "QueryAndPhysics")
          (bind (_direction _scaletrack) (`Timeline|ScaleGraph` :!via `PlayFromStart`)
            (:`Update`
              (bind _returnvalue (`KismetMathLibrary.Lerp` 0.1 22.0 _scaletrack))
              (`SceneComponent.SetRelativeScale3D` _hatch (`KismetMathLibrary.MakeVector` _returnvalue _returnvalue 0.1)))
            (:`Finished`
              (goto _label :!via `Close`))))))))

(fn `UserConstructionScript`
  (`PrimitiveComponent.SetCollisionEnabled` (`self.Hatch`) "NoCollision"))